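; Enemy spawner actor that spawns a requested number of enemies as a wave, split into batches.
; SpawnWave stores the count, then SpawnBatch spawns up to BatchSize EnemyStub actors and calls itself after a fixed delay until none remain.
; GetRandomSpawnPoint places each at a random flat XY offset within a square around the spawner, with fixed rotation and heavily reduced scale.
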(event Custom|SpawnWave
  (params (EnemiesToSpawn :type Integer))
  (Variables|Default|SetEnemies%20to%20Spawn EnemiesToSpawn)
  (CallFunction|SpawnBatch))

(event Custom|SpawnBatch
  (bind _enemies_to_spawn (Variables|Default|GetEnemies%20to%20Spawn))
  (Variables|Default|SetSpawned 0)
  (while (and (< (Variables|Default|GetSpawned) (Variables|Default|GetBatchSize)) (> _enemies_to_spawn 0))
    (Game|SpawnActorfromClass "/Game/Player/EnemyStub.EnemyStub_C" (CallFunction|GetRandomSpawnPoint) "AdjustIfPossibleButAlwaysSpawn" 0 0)
    (Math|Integer|IncrementInt (Variables|Default|GetSpawned)
      (:%20%20
        (Math|Integer|DecrementInt (Variables|Default|GetEnemies%20to%20Spawn)))))
  (if (> _enemies_to_spawn 0)
    (Utilities|FlowControl|Delay 5.0)
    (CallFunction|SpawnBatch)))

(fn ConstructionScript)

(fn GetRandomSpawnPoint
  (return (Math|Transform|MakeTransform (+ (Math|Vector|MakeVector (Math|Random|RandomFloatinRange -1e+03 1e+03) (Math|Random|RandomFloatinRange -1e+03 1e+03) 0.0) (Transformation|GetWorldLocation (Variables|Default|GetDefaultSceneRoot))) "0, 0, 0" "0.031250,0.031250,0.031250")))