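; Player state Blueprint that holds a player's name and HP and overrides CopyProperties to hand data to a replacement player state.
; The override casts the new state and copies PlayerName into it, but assigns max and current HP back onto itself, so HP is not transferred.
; BeginPlay and CopyProperties contain leftover debug prints.
; An unconnected chain with a broken game instance cast would set PlayerName but never runs.
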(event EventBeginPlay
  (Development|PrintString "nowy" false false))

(event EventTick
  (params (DeltaSeconds :type Float%20%28single-precision%29)))

(event EventCopyProperties
  (params (NewPlayerState :type Player%20State%20Object%20Reference))
  (Development|PrintString "sadfgnmtyhrgefdasg")
  (bind _asplayer_state (Utilities|Casting|CastToplayer_state NewPlayerState))
  (Variables|player_state_C|Setplayer_name _asplayer_state (Variables|Default|Getplayer_name))
  (Variables|Default|Setplayer_max_hp (Variables|Default|Getplayer_max_hp))
  (Variables|Default|Setplayer_current_hp (Variables|Default|Getplayer_current_hp)))

(fn ConstructionScript)