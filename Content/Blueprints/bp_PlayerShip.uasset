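; Player-controlled ship pawn that extends a parent ship class with input, a mounted turret and a HUD.
; Turn axis and arrow-key gear inputs route through server events into the Turn, GearUp and GearDown calls.
; On BeginPlay the authority spawns a player turret, attaches it to the body socket and passes it turret parameters, while the locally controlled client creates the HUD widget.
; Tick prints hit points on the authority.
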(event Custom|ServerSpawnTurret
  (bind _self self)
  (bind _arrow (Variables|Default|GetArrow))
  (bind _returnvalue (Transformation|GetWorldTransform _arrow))
  (Utilities|FlowControl|Sequence
    (:then_0
      ;[1 1 1] Spawning and caching the turret
      (Networking|SwitchHasAuthority
        (:Authority
          (Utilities|FlowControl|Sequence
            (:then_0
              (bind _returnvalue_2 (Game|SpawnActorfromClass "/Game/Turret/BP_TurretPlayer.BP_TurretPlayer_C" (Math|Transform|MakeTransform (.location _returnvalue) (.rotation _returnvalue) "0.300000,0.300000,0.300000") "AlwaysSpawn" _self _self))
              (bind _output_get (Variables|Default|SetGun _returnvalue_2))
              (Transformation|AttachComponentToComponent _output_get (Variables|Default|GetSpaceshipBody) "TurretSocket" "KeepWorld" "SnapToTarget" "KeepWorld" true))
            (:then_1
              (bind _asbp_turret_player (Utilities|Casting|CastToBP_TurretPlayer (Variables|Default|GetGun)))
              (Variables|/Game/Turret/BP_Turret.BP_Turret_C|SetParameters _asbp_turret_player (Variables|Default|GetTurretParameters)))))))))

(event Custom|serverGearDown
  ;[1 1 1] Gear handling
  (Class|CppSpaceship|GearDown))

(event Custom|LocalCreateHud
  (if (Pawn|IsLocallyControlled)
    (bind _asplayer_controller (Utilities|Casting|CastToPlayerController (Pawn|GetController)))
    (bind _returnvalue (UserInterface|CreateWidget "/Game/gui/Minimap/HUD_Widget.HUD_Widget_C" _asplayer_controller))
    (bind _output_get (Variables|Default|SetHUD_Widget _returnvalue))
    (UserInterface|Viewport|AddtoViewport _output_get 0)))

(event Custom|serverTurn
  (params (Axis%20Value :type Float%20%28single-precision%29))
  ;[1 1 1] Turn handling
  (CallFunction|Turn Axis%20Value))

(event Custom|serverGearUp
  ;[1 1 1] Gear handling
  (Class|CppSpaceship|GearUp))

(event EventBeginPlay
  (|CallParentFunction)
  (Networking|SwitchHasAuthority
    (:Authority
      (CallFunction|ServerSpawnTurret))
    (:Remote
      _))
  (CallFunction|LocalCreateHud))

(event EventTick
  (params (DeltaSeconds :type Float%20%28single-precision%29))
  (|CallParentFunction DeltaSeconds)
  (Networking|SwitchHasAuthority
    (:Authority
      (Development|PrintString (Utilities|String|ToString(Float) (Variables|Default|GetHitPoints))))))

(event Input|ActionEvents|InputActionArrowDown
  (params (Key :type Key%20Structure :default "None"))
  ;[1 1 1] Gear handling
  (:Pressed
    (CallFunction|ServerGearDown)))

(event Input|ActionEvents|InputActionArrowUp
  (params (Key :type Key%20Structure :default "None"))
  ;[1 1 1] Gear handling
  (:Pressed
    (CallFunction|ServerGearUp)))

(event Input|AxisEvents|InputAxisTurn
  (params (AxisValue :type Float%20%28single-precision%29))
  ;[1 1 1] Turn handling
  (CallFunction|ServerTurn AxisValue))

(fn ConstructionScript
  (|CallParentFunction))