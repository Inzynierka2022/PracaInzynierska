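; Exploding turret bullet that damages a spaceship on direct hit and deals area damage when destroyed, tagged with its team.
; The Box triggers the hit, ignoring the owner, while the Sphere keeps a list of player ships in blast range.
; On Destroyed it damages every listed ship, draws a debug sphere and spawns the explosion through the particle-and-sound replicator actor.
; All of this logic runs only on the authority.
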(event OnComponentBeginOverlap(Box)
  (params (OverlappedComponent :type Primitive%20Component%20Object%20Reference) (OtherActor :type Actor%20Object%20Reference) (OtherComp :type Primitive%20Component%20Object%20Reference) (OtherBodyIndex :type Integer) (bFromSweep :type Boolean) (SweepResult :type Hit%20Result%20Structure%20%28by%20ref%29))
  (Networking|SwitchHasAuthority
    (:Authority
      (if (!= OtherActor (Components|GetOwner))
        (bind _asbp_spaceship (Utilities|Casting|CastTobp_Spaceship OtherActor))
        (Default|TakeDamage _asbp_spaceship (Variables|Default|GetDamage) (Variables|Default|GetTeamId))
        (Actor|DestroyActor)))))

(event OnComponentBeginOverlap(Sphere)
  (params (OverlappedComponent :type Primitive%20Component%20Object%20Reference) (OtherActor :type Actor%20Object%20Reference) (OtherComp :type Primitive%20Component%20Object%20Reference) (OtherBodyIndex :type Integer) (bFromSweep :type Boolean) (SweepResult :type Hit%20Result%20Structure%20%28by%20ref%29))
  (Networking|SwitchHasAuthority
    (:Authority
      (bind _asbp_player_ship (Utilities|Casting|CastTobp_PlayerShip OtherActor))
      (Utilities|Array|AddUnique (Variables|Default|GetPlayersInExplosionRange) _asbp_player_ship))))

(event OnComponentEndOverlap(Sphere)
  (params (OverlappedComponent :type Primitive%20Component%20Object%20Reference) (OtherActor :type Actor%20Object%20Reference) (OtherComp :type Primitive%20Component%20Object%20Reference) (OtherBodyIndex :type Integer))
  (Networking|SwitchHasAuthority
    (:Authority
      (bind _asbp_player_ship (Utilities|Casting|CastTobp_PlayerShip OtherActor))
      (Utilities|Array|RemoveItem (Variables|Default|GetPlayersInExplosionRange) _asbp_player_ship))))

(event EventBeginPlay
  (|CallParentFunction))

(event EventDestroyed
  (bind _sphere (Variables|Default|GetSphere))
  (bind _returnvalue (Transformation|GetWorldLocation _sphere))
  (Networking|SwitchHasAuthority
    (:Authority
      (for _array_element (Variables|Default|GetPlayersInExplosionRange)
        (bind _asbp_spaceship (Utilities|Casting|CastTobp_Spaceship _array_element))
        (Default|TakeDamage _asbp_spaceship (Variables|Default|GetDamage) (Variables|Default|GetTeamId))
        (Development|PrintString (Utilities|GetDisplayName _asbp_spaceship)))
      (Rendering|Debug|DrawDebugSphere _returnvalue (Components|Sphere|GetScaledSphereRadius _sphere) 12 "(R=1.000000,G=0.000000,B=0.013838,A=1.000000)" 5.0)
      (bind _returnvalue_2 (Actor|GetActorOfClass "/Game/Sounds/a_particle_and_sound_replicator.a_particle_and_sound_replicator_C"))
      (Default|SpawnEmitter _returnvalue_2 "/Game/MyParticleSystems/P_Explosion.P_Explosion" _returnvalue (* (Transformation|GetActorScale3D) 10)))))

(fn ConstructionScript
  (|CallParentFunction))