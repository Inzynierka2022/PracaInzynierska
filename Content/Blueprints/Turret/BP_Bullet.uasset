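; Turret projectile that damages spaceships on overlap and plays a gunshot sound when spawned.
; Construction sets the projectile movement speed and derives lifespan from range divided by speed.
; Overlaps are handled on the authority only, skipping the owner, passing damage and team ID to the ship before destroying the bullet.
; The impact emitter spawns through a shared particle-and-sound replicator actor found in the level.
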(event Custom|Event%20Effect
  (params (Location :type Vector))
  (bind _returnvalue (Math|Float|MakeLiteralFloat 0.1))
  (bind _returnvalue_2 (Actor|GetActorOfClass "/Game/Sounds/a_particle_and_sound_replicator.a_particle_and_sound_replicator_C"))
  (Utilities|IsValid _returnvalue_2
    (:Is%20Valid
      (Default|SpawnEmitter _returnvalue_2 "/Game/MyParticleSystems/P_Bum.P_Bum" Location (Math|Vector|MakeVector _returnvalue _returnvalue _returnvalue)))))

(event Collision|EventActorBeginOverlap
  (params (OtherActor :type Actor%20Object%20Reference))
  (Networking|SwitchHasAuthority
    (:Authority
      (if (!= OtherActor (Components|GetOwner))
        (bind _asbp_spaceship (Utilities|Casting|CastTobp_Spaceship OtherActor))
        (CallFunction|EventEffect (Transformation|GetWorldLocation (Variables|Default|GetScene)))
        (Default|TakeDamage _asbp_spaceship (Variables|Default|GetDamage) (Variables|Default|GetTeamId))
        (Actor|DestroyActor)))))

(event EventBeginPlay
  (Audio|PlaySoundatLocation "/Game/Sounds/9mm-pistol-shot-6349_Cue.9mm-pistol-shot-6349_Cue" (Transformation|GetWorldLocation (Variables|Default|GetBulletMesh)) "0, 0, 0" 0.1 1.0 0.0 0 0 0))

(fn ConstructionScript
  (bind _output_get (Variables|/Script/Engine.ProjectileMovementComponent|SetInitialSpeed (Variables|Default|GetProjectileMovement) (Variables|Default|GetSpeed)))
  (Actor|SetLifeSpan (/ (Variables|Default|GetRange) _output_get)))