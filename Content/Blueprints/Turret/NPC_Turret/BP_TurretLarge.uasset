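; BP_TurretLarge is a large NPC turret that adds a one-shot sniper attack to its parent turret's normal behavior.
; ChangeToSniperMode stores a target location; the authority-only, pause-aware Tick then rotates toward it instead of running the parent Tick.
; Once the top aligns within a degree in 2D, SniperFire spawns boosted-damage bullets from every arrow component, ranged just past the target, and normal behavior resumes.
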(event Custom|ChangeToSniperMode
  (params (NewParam :type Vector))
  (Variables|Default|SetPlayerLocation NewParam)
  (Variables|Default|SetSniperMode true))

(event EventTick
  (params (DeltaSeconds :type Float%20%28single-precision%29))
  (Networking|SwitchHasAuthority
    (:Authority
      (bind _asgameplay_gamemode (Utilities|Casting|CastToGameplayGamemode (Game|GetGameMode)))
      (if (not (Variables|/Game/Blueprints/GameplayGamemode.GameplayGamemode_C|GetGamePaused _asgameplay_gamemode))
        (if (Variables|Default|GetSniperMode)
          (CallFunction|RotateTowards (Variables|Default|GetPlayerLocation))
          (if (< (Class|KismetMathLibrary|DegAcos (Math|Vector|DotProduct (Class|KismetMathLibrary|VectorNormal2D (Math|Vector|GetForwardVector (Variables|Default|GetRotatableTop)) 0.0001) (Class|KismetMathLibrary|VectorNormal2D (- (Variables|Default|GetPlayerLocation) (Transformation|GetWorldLocation (Variables|Default|GetDefaultSceneRoot))) 0.0001))) 1.0)
            (CallFunction|SniperFire)
            (Variables|Default|SetSniperMode false))
          (else
            (|CallParentFunction DeltaSeconds)))))))

(fn ConstructionScript
  (|CallParentFunction))

(fn SniperFire
  (bind _parameters (Variables|Default|GetParameters))
  (for _array_element (Actor|GetComponentsByClass "/Script/Engine.ArrowComponent")
    (Game|SpawnActorfromClass "/Game/Blueprints/Turret/BP_Bullet.BP_Bullet_C" (Math|Transform|MakeTransform (.location (Transformation|GetWorldTransform _array_element)) (.rotation (Transformation|GetWorldTransform _array_element)) "1,1,1") "Undefined" (Components|GetOwner) (Variables|Default|GetTeam) (* 4 (.Value (Utilities|Map|Find (Variables|/Game/Blueprints/Turret/BP_TurretParameters.BP_TurretParameters_C|GetCurrentParameters _parameters) "NewEnumerator2"))) (Variables|/Game/Blueprints/Turret/BP_TurretParameters.BP_TurretParameters_C|GetBulletSpeed _parameters) (+ (Math|Vector|Distance(Vector) (Transformation|GetWorldLocation (Variables|Default|GetDefaultSceneRoot)) (Variables|Default|GetPlayerLocation)) 5e+01) 0)))