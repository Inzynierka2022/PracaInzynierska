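; Player-owned turret that aims at the mouse cursor and supports leveled stat upgrades.
; Each tick, a locally controlled owner traces under the cursor and rotates the turret, directly with authority or through RequestRotateToMouse on remote clients.
; Upgrades linearly interpolate a parameter between its base and max values by clamped level, store it as current, and also update magazine size for one parameter type.
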(event Custom|RequestRotateToMouse
  (params (MousePosition :type Vector))
  (CallFunction|RotateTowards MousePosition))

(event Custom|Upgrade
  (params (Type :type UpgradeEnum%20Enum :default "NewEnumerator0") (Level :type Integer))
  (CallFunction|UpgradeParameters Type Level))

(event EventBeginPlay
  (|CallParentFunction))

(event EventTick
  (params (DeltaSeconds :type Float%20%28single-precision%29))
  (|CallParentFunction DeltaSeconds)
  (Networking|SwitchHasAuthority
    (:Authority
      (bind _aspawn (Utilities|Casting|CastToPawn (Components|GetOwner)))
      (if (Pawn|IsLocallyControlled _aspawn)
        (bind _aspawn_2 (Utilities|Casting|CastToPawn (Components|GetOwner)))
        (bind _asplayer_controller (Utilities|Casting|CastToPlayerController (Pawn|GetController _aspawn_2)))
        (CallFunction|RotateTowards (.Location (Collision|BreakHitResult (.HitResult (Game|Player|GetHitResultUnderCursorbyChannel _asplayer_controller "TraceTypeQuery3" true)))))))
    (:Remote
      (bind _aspawn_3 (Utilities|Casting|CastToPawn (Components|GetOwner)))
      (if (Pawn|IsLocallyControlled _aspawn_3)
        (bind _asplayer_controller_2 (Utilities|Casting|CastToPlayerController (Pawn|GetController _aspawn_3)))
        (CallFunction|RequestRotatetoMouse (.Location (Collision|BreakHitResult (.HitResult (Game|Player|GetHitResultUnderCursorbyChannel _asplayer_controller_2 "TraceTypeQuery3" true)))))))))

(fn ConstructionScript
  (|CallParentFunction))

(fn UpgradeParameters
  (params (Type :type UpgradeEnum%20Enum :default "NewEnumerator0") (Level :type Integer))
  (bind _parameters (Variables|Default|GetParameters))
  (bind _result (CallFunction|CalculateUpgrade (.Value (Utilities|Map|Find (Variables|/Game/Blueprints/Turret/BP_TurretParameters.BP_TurretParameters_C|GetBaseParameters _parameters) Type)) (.Value (Utilities|Map|Find (Variables|/Game/Blueprints/Turret/BP_TurretParameters.BP_TurretParameters_C|GetMaxParameters _parameters) Type)) Level))
  (Utilities|Map|Add (Variables|/Game/Blueprints/Turret/BP_TurretParameters.BP_TurretParameters_C|GetCurrentParameters _parameters) Type _result)
  (if (Utilities|Enum|Equal(Enum) Type "NewEnumerator7")
    (Variables|Default|SetMagSize (Math|Float|Truncate _result))))

(fn CalculateUpgrade
  (params (Min :type Float%20%28single-precision%29) (Max :type Float%20%28single-precision%29) (Level :type Integer))
  (bind _maxupgradelevel (Variables|Default|GetMaxUpgradeLevel))
  (return (+ (* (Math|Integer|Clamp(Integer) Level 0 _maxupgradelevel) (/ (- Max Min) (Math|Conversions|ToFloat(Integer) _maxupgradelevel))) Min)))