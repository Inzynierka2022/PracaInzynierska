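; Automatic turret that, on the server, tracks the nearest player ship or space station and fires on it.
; Overlap events maintain PlayersInRange, from which ChooseTarget picks the closest SpaceshipBody location, flattened to Z=0, or a point ahead of the base when empty.
; Tick rotates toward that point and calls TryShoot if a target is listed within 1000 units, otherwise StopShooting.
; The construction script's sphere-radius adjustment is disconnected.
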(event Collision|EventActorBeginOverlap
  (params (OtherActor :type Actor%20Object%20Reference))
  (bind _playersinrange (Variables|Default|GetPlayersInRange))
  (Networking|SwitchHasAuthority
    (:Authority
      (bind _asbp_player_ship (Utilities|Casting|CastTobp_PlayerShip OtherActor)
        (:then
          (Utilities|Array|AddUnique _playersinrange _asbp_player_ship))
        (:CastFailed
          (bind _asbp_space_station (Utilities|Casting|CastTobp_SpaceStation OtherActor))
          (Utilities|Array|AddUnique _playersinrange _asbp_space_station))))))

(event Collision|EventActorEndOverlap
  (params (OtherActor :type Actor%20Object%20Reference))
  (Networking|SwitchHasAuthority
    (:Authority
      (bind _asbp_player_ship (Utilities|Casting|CastTobp_PlayerShip OtherActor)
        (:then
          (Utilities|Array|RemoveItem (Variables|Default|GetPlayersInRange) _asbp_player_ship))
        (:CastFailed
          (bind _asbp_space_station (Utilities|Casting|CastTobp_SpaceStation OtherActor))
          (Utilities|Array|RemoveItem (Variables|Default|GetPlayersInRange) _asbp_space_station))))))

(event EventTick
  (params (DeltaSeconds :type Float%20%28single-precision%29))
  (bind _playerlocation (Variables|Default|GetPlayerLocation))
  (|CallParentFunction DeltaSeconds)
  (Networking|SwitchHasAuthority
    (:Authority
      (CallFunction|ChooseTarget)
      (CallFunction|RotateTowards _playerlocation)
      (if (and (< (Math|Vector|Distance(Vector) _playerlocation (Transformation|GetActorLocation)) 1e+03) (> (Utilities|Array|Length (Variables|Default|GetPlayersInRange)) 0))
        (CallFunction|TryShoot)
        (else
          (CallFunction|StopShooting))))))

(fn ConstructionScript
  (Networking|SwitchHasAuthority))

(fn ChooseTarget
  (bind _staticbottom (Variables|Default|GetStaticBottom))
  (bind _returnvalue (Math|Vector|GetForwardVector _staticbottom))
  (bind _returnvalue_2 (Transformation|GetWorldLocation _staticbottom))
  (bind _returnvalue_3 (* _returnvalue 1e+02))
  (bind _returnvalue_4 (+ _returnvalue_2 _returnvalue_3))
  (if (> (Utilities|Array|Length (Variables|Default|GetPlayersInRange)) 0)
    (for (_array_element _array_index) (Variables|Default|GetPlayersInRange)
      (if (== _array_index 0)
        (Variables|Default|SetClosestDistance (Math|Vector|Distance(Vector) (Transformation|GetWorldLocation (Variables|/Game/Blueprints/bp_Spaceship.bp_Spaceship_C|GetSpaceshipBody _array_element)) (Transformation|GetWorldLocation (Variables|Default|GetDefaultSceneRoot))) :!label _label)
        (Variables|Default|SetPlayerLocation (Math|Vector|MakeVector (.X (Math|Vector|BreakVector (Transformation|GetWorldLocation (Variables|/Game/Blueprints/bp_Spaceship.bp_Spaceship_C|GetSpaceshipBody _array_element)))) (.Y (Math|Vector|BreakVector (Transformation|GetWorldLocation (Variables|/Game/Blueprints/bp_Spaceship.bp_Spaceship_C|GetSpaceshipBody _array_element)))) 0.0))
        (elif (< (Math|Vector|Distance(Vector) (Transformation|GetWorldLocation (Variables|/Game/Blueprints/bp_Spaceship.bp_Spaceship_C|GetSpaceshipBody _array_element)) (Transformation|GetWorldLocation (Variables|Default|GetDefaultSceneRoot))) (Variables|Default|GetClosestDistance))
          (goto _label))))
    (else
      (Variables|Default|SetPlayerLocation (Math|Vector|MakeVector (.x _returnvalue_4) (.y _returnvalue_4) 0.0)))))