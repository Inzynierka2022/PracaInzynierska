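; BP_Turret is a server-authoritative turret that fires BP_Bullet projectiles while IsShooting is set and the game is unpaused.
; Tick drives TryShoot, with Delays gating fire rate and magazine reloads using values from a Parameters stat map.
; Fire spawns a team-tagged bullet from every arrow component with random yaw spread.
; RotateTowards turns the top toward a target at constant speed within an angle limit.
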(event Custom|Shoot
  (bind _parameters (Variables|Default|GetParameters))
  (if (> (Variables|Default|GetBulletsInMag) 0)
    (CallFunction|Fire)
    (Variables|Default|SetCanShoot false)
    (bind _result (Math|Integer|DecrementInt (Variables|Default|GetBulletsInMag))
      (:%20%20
        (if (> _result 0)
          (Utilities|FlowControl|Delay (.Value (Utilities|Map|Find (Variables|/Game/Blueprints/Turret/BP_TurretParameters.BP_TurretParameters_C|GetCurrentParameters (Variables|Default|GetParameters)) "NewEnumerator0")))
          (else
            (Variables|Default|SetIsReloading true)
            (Utilities|FlowControl|Delay (Variables|/Game/Blueprints/Turret/BP_TurretParameters.BP_TurretParameters_C|GetMagReloadTime _parameters))
            (Variables|Default|SetIsReloading false)
            (Variables|Default|SetBulletsInMag (Math|Float|Truncate (.Value (Utilities|Map|Find (Variables|/Game/Blueprints/Turret/BP_TurretParameters.BP_TurretParameters_C|GetCurrentParameters _parameters) "NewEnumerator7"))))))
        (Variables|Default|SetCanShoot true)))))

(event Custom|TryShoot
  (if (Variables|Default|GetCanShoot)
    (bind _returnvalue (Utilities|Time|SetTimerbyEvent (delegate Custom|Shoot) (.Value (Utilities|Map|Find (Variables|/Game/Blueprints/Turret/BP_TurretParameters.BP_TurretParameters_C|GetCurrentParameters (Variables|Default|GetParameters)) "NewEnumerator0"))))
    (CallFunction|Shoot)))

(event Custom|StopShooting
  (Utilities|Time|ClearandInvalidateTimerbyHandle (stale Custom|TryShoot _returnvalue)))

(event EventBeginPlay
  (Networking|SwitchHasAuthority
    (:Authority
      (Variables|Default|SetBulletsInMag (Math|Float|Truncate (.Value (Utilities|Map|Find (Variables|/Game/Blueprints/Turret/BP_TurretParameters.BP_TurretParameters_C|GetCurrentParameters (Variables|Default|GetParameters)) "NewEnumerator7")))))))

(event EventTick
  (params (DeltaSeconds :type Float%20%28single-precision%29))
  (Networking|SwitchHasAuthority
    (:Authority
      (bind _asgameplay_gamemode (Utilities|Casting|CastToGameplayGamemode (Game|GetGameMode)))
      (if (not (Variables|/Game/Blueprints/GameplayGamemode.GameplayGamemode_C|GetGamePaused _asgameplay_gamemode))
        (if (Variables|Default|GetIsShooting)
          (CallFunction|TryShoot)
          (else
            (CallFunction|StopShooting)))))))

(fn ConstructionScript)

(fn Fire
  (bind _parameters (Variables|Default|GetParameters))
  (bind _parameters_2 (Variables|Default|GetParameters))
  (bind _parameters_3 (Variables|Default|GetParameters))
  (bind _bulletsize (Variables|/Game/Blueprints/Turret/BP_TurretParameters.BP_TurretParameters_C|GetBulletSize _parameters_3))
  (bind _currentparameters (Variables|/Game/Blueprints/Turret/BP_TurretParameters.BP_TurretParameters_C|GetCurrentParameters _parameters))
  (bind _currentparameters_2 (Variables|/Game/Blueprints/Turret/BP_TurretParameters.BP_TurretParameters_C|GetCurrentParameters _parameters_2))
  (bind _value (Utilities|Map|Find _currentparameters_2 "NewEnumerator3"))
  (for _array_element (Actor|GetComponentsByClass "/Script/Engine.ArrowComponent")
    (Game|SpawnActorfromClass "/Game/Blueprints/Turret/BP_Bullet.BP_Bullet_C" (Math|Transform|MakeTransform (.location (Transformation|GetWorldTransform _array_element)) (Math|Rotator|CombineRotators (.rotation (Transformation|GetWorldTransform _array_element)) (Math|Rotator|MakeRotator 0.0 0.0 (Math|Random|RandomFloatinRange (* _value -1.0) _value))) (Math|Vector|MakeVector _bulletsize _bulletsize _bulletsize)) "Undefined" (Components|GetOwner) (Variables|Default|GetTeam) (.Value (Utilities|Map|Find _currentparameters "NewEnumerator2")) (Variables|/Game/Blueprints/Turret/BP_TurretParameters.BP_TurretParameters_C|GetBulletSpeed _parameters) (.Value (Utilities|Map|Find _currentparameters "NewEnumerator1")) 0)))

(fn RotateTowards
  (params (Target :type Vector%20%28by%20ref%29))
  (bind _parameters (Variables|Default|GetParameters))
  (bind _anglelimit (Variables|/Game/Blueprints/Turret/BP_TurretParameters.BP_TurretParameters_C|GetAngleLimit _parameters))
  (Transformation|SetRelativeRotation (Variables|Default|GetRotatableTop) (Class|KismetMathLibrary|RInterptoConstant (Variables|/Script/Engine.SceneComponent|GetRelativeRotation (Variables|Default|GetRotatableTop)) (Math|Rotator|MakeRotator 0.0 0.0 (Math|Float|ClampAngle (.yaw (Math|Rotator|MakeRotfromX (Math|Transform|InverseTransformLocation (Transformation|GetActorTransform) Target))) (- 0.0 _anglelimit) _anglelimit)) (Utilities|Time|GetWorldDeltaSeconds) (.Value (Utilities|Map|Find (Variables|/Game/Blueprints/Turret/BP_TurretParameters.BP_TurretParameters_C|GetCurrentParameters (Variables|Default|GetParameters)) "NewEnumerator5"))) false false))