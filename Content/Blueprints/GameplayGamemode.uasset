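; Game mode for a multiplayer ship wave game, tracking players, waves and the win or loss result.
; A Tick countdown starts each wave through a spawned BP_EnemySpawner, and enemy kill counts end it.
; Between waves it respawns spectators, waits for every player's upgrade-finished event, resets ships and raises the level.
; Dead players become spectators until none remain alive, and the outcome is written to GameplayGameState.
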(event Custom|ManageUpgrades
  (Variables|Default|SetPlayersReady 0)
  (for _array_element (Variables|Default|GetplayerControllers)
    (bind _asin_game_player_controller (Utilities|Casting|CastToInGamePlayerController _array_element))
    (Default|Upgrade _asin_game_player_controller)
    (EventDispatchers|BindEventtoUpgradesFinished _asin_game_player_controller (delegate Custom|PlayerReady))))

(event Custom|UpgradesFinished
  (Variables|Default|SetUpgrading false)
  (bind _outactors (Actor|GetAllActorsOfClass "/Game/Blueprints/bp_PlayerShip.bp_PlayerShip_C"))
  (for _array_element _outactors
    (Class|CppSpaceship|Stop _array_element))
  (CallFunction|ResetPlayers)
  (Math|Integer|IncrementInt (Variables|Default|GetLevel)
    (:%20%20
      (CallFunction|StartCountDown))))

(event Custom|removePlayerController
  (params (NewParam :type In%20Game%20Player%20Controller%20Object%20Reference))
  (Utilities|Array|RemoveItem (Variables|Default|GetplayerControllers) NewParam)
  (CallFunction|UpdateAll self))

(event Custom|StartGame
  (Networking|SwitchHasAuthority
    (:Authority
      (Variables|Default|SetPlayersAlive (Utilities|Array|Length (Variables|Default|GetplayerControllers)))
      (CallFunction|StartCountDown))))

(event Custom|GameWon
  (bind _asgameplay_game_state (Utilities|Casting|CastToGameplayGameState (Game|GetGameState)))
  (Variables|/Game/Blueprints/GameplayGameState.GameplayGameState_C|SetGameFinished _asgameplay_game_state true)
  (Variables|/Game/Blueprints/GameplayGameState.GameplayGameState_C|SetGameWon _asgameplay_game_state true))

(event Custom|GameLost
  (bind _asgameplay_game_state (Utilities|Casting|CastToGameplayGameState (Game|GetGameState)))
  (Variables|/Game/Blueprints/GameplayGameState.GameplayGameState_C|SetGameFinished _asgameplay_game_state true)
  (Variables|/Game/Blueprints/GameplayGameState.GameplayGameState_C|SetGameWon _asgameplay_game_state false))

(event Custom|WaveEnded
  (Networking|SwitchHasAuthority
    (:Authority
      (if (< (Variables|Default|GetLevel) (Variables|Default|GetMaxLevel))
        (if (not (Variables|Default|GetUpgrading))
          (CallFunction|RespawnPlayers)
          (CallFunction|ManageUpgrades)
          (Variables|Default|SetUpgrading true))
        (else
          (CallFunction|GameWon))))))

(event Custom|StartCountdown
  (Variables|Default|SetCountdownTimer 0.5)
  (Variables|Default|SetCountdown true)
  (Variables|Default|SetGamePaused true))

(event Custom|StopCountdown
  (Variables|Default|SetCountdown false)
  (Variables|Default|SetGamePaused false)
  (CallFunction|SpawnEnemyWave))

(event Custom|SpawnPlayer
  (params (PlayerController :type Player%20Controller%20Object%20Reference))
  (bind _asin_game_player_controller (Utilities|Casting|CastToInGamePlayerController PlayerController))
  (Utilities|IsValid (Pawn|GetControlledPawn _asin_game_player_controller)
    (:Is%20Valid
      (Actor|DestroyActor (Pawn|GetControlledPawn _asin_game_player_controller)))
    (:Is%20Not%20Valid
      _))
  (bind _returnvalue (Game|SpawnActorfromClass (.playershipclass (Variables|/Game/Blueprints/InGamePlayerController.InGamePlayerController_C|GetplayerInfo _asin_game_player_controller)) (Transformation|GetActorTransform (Class|GameModeBase|FindPlayerStart _asin_game_player_controller)) "AdjustIfPossibleButAlwaysSpawn" 0 0))
  (Pawn|Possess _asin_game_player_controller _returnvalue))

(event Custom|PlayerReady
  (bind _playercontrollers (Variables|Default|GetplayerControllers))
  (bind _returnvalue (Utilities|Array|Length _playercontrollers))
  (bind _result (Math|Integer|IncrementInt (Variables|Default|GetPlayersReady))
    (:%20%20
      ;[1 1 1] Debug printing
      (Development|PrintString (Utilities|String|Append (Utilities|String|ToString(Integer) _result) "/" (Utilities|String|ToString(Integer) _returnvalue)))
      (if (== _result _returnvalue)
        (CallFunction|UpgradesFinished)))))

(event Custom|SpawnEnemyWave
  (bind _enemiesspawned (Default|SpawnWave (Variables|Default|GetSpawner) (Variables|Default|GetLevel)))
  (Variables|Default|SetTotalEnemiesLeft _enemiesspawned))

(event Custom|EnemyDestroyed
  (bind _result (Math|Integer|DecrementInt (Variables|Default|GetEnemiesLeft))
    (:%20%20
      (bind _result_2 (Math|Integer|DecrementInt (Variables|Default|GetTotalEnemiesLeft))
        (:%20%20
          (Development|PrintString (Utilities|String|Append "Enemies left: " (Utilities|String|ToString(Integer) _result)))
          (if (== _result_2 0)
            (CallFunction|WaveEnded)))))))

(event Custom|EnemySpawned
  (bind _result (Math|Integer|IncrementInt (Variables|Default|GetEnemiesLeft))
    (:%20%20
      (Development|PrintString (Utilities|String|Append "Enemies left: " (Utilities|String|ToString(Integer) _result))))))

(event Custom|SpectatorSpawnRequest
  (params (PlayerController :type Player%20Controller%20Object%20Reference))
  (bind _result (Math|Integer|DecrementInt (Variables|Default|GetPlayersAlive))
    (:%20%20
      (if (> _result 0)
        (Utilities|IsValid PlayerController
          (:Is%20Valid
            (Networking|SwitchHasAuthority
              (:Authority
                (bind _returnvalue (Game|SpawnActorfromClass "/Game/Blueprints/BP_Spectator.BP_Spectator_C" (Math|Transform|MakeTransform "800.000000, 0,0.000000") "Undefined" 0 0))
                (Utilities|FlowControl|Delay 0.2)
                (Pawn|Possess PlayerController _returnvalue)))))
        (else
          (CallFunction|GameLost))))))

(event Custom|updateAll
  (bind _playerinfos (Variables|Default|GetplayerInfos))
  ;[1 1 1] updateAllPlayer info on new player join
  (Utilities|Array|Clear (Variables|Default|GetplayerInfos))
  (for _array_element (Variables|Default|GetplayerControllers)
    (bind _asin_game_player_controller (Utilities|Casting|CastToInGamePlayerController _array_element))
    (Utilities|Array|Add _playerinfos (Variables|/Game/Blueprints/InGamePlayerController.InGamePlayerController_C|GetplayerInfo _asin_game_player_controller)))
  (Development|PrintString (Utilities|String|ToString(Integer) (Utilities|Array|Length _playerinfos)) false false "(R=1.000000,G=0.838870,B=0.000000,A=1.000000)" 1e+01)
  (for _array_element_2 _playerinfos
    (Development|PrintString (Utilities|String|ToString(Text) (Utilities|Text|FormatText "{player} : {ship}" (.PlayerName (Utilities|Struct|BreakPlayerInfo _array_element_2)) (.PlayerShipName (Utilities|Struct|BreakPlayerInfo _array_element_2)))) false false "(R=0.000000,G=0.660000,B=1.000000,A=1.000000)" 1e+01))
  (Development|PrintString (Utilities|String|ToString(Integer) (Utilities|Array|Length (Variables|Default|GetplayerInfos))) false false "(R=1.000000,G=0.838870,B=0.000000,A=1.000000)" 1e+01)
  (CallFunction|CallUpdatePlayersLists self))

(event Custom|callUpdatePlayersLists
  (bind _playercontrollers (Variables|Default|GetplayerControllers))
  ;[1 1 1] updateAllPlayersLists
  (for _array_element _playercontrollers
    (bind _asin_game_player_controller (Utilities|Casting|CastToInGamePlayerController _array_element))
    (Default|UpdatePlayerList _asin_game_player_controller (Variables|Default|GetplayerInfos)))
  (Development|PrintString (Utilities|String|ToString(Text) (Utilities|Text|FormatText "player controllers {a}" (Utilities|Array|Length _playercontrollers))) false false "(R=0.000000,G=0.660000,B=1.000000,A=1.000000)" 1e+01))

(event Custom|RespawnPlayers
  (bind _playercontrollers (Variables|Default|GetplayerControllers))
  (Variables|Default|SetPlayersAlive (Utilities|Array|Length _playercontrollers))
  (for _array_element _playercontrollers
    (bind _asin_game_player_controller (Utilities|Casting|CastToInGamePlayerController _array_element))
    (bind _asbp_spectator (Utilities|Casting|CastToBP_Spectator (Pawn|GetControlledPawn _asin_game_player_controller)))
    (Actor|DestroyActor _asbp_spectator)
    (CallFunction|SpawnPlayer _asin_game_player_controller)
    (Default|RestoreParametersonRespawn _asin_game_player_controller)))

(event EventTick
  (params (DeltaSeconds :type Float%20%28single-precision%29))
  (if (Variables|Default|GetCountdown)
    (bind _output_get (Variables|Default|SetCountdownTimer (- (Variables|Default|GetCountdownTimer) DeltaSeconds)))
    (if (<= _output_get 0.0)
      (CallFunction|StopCountDown))))

(event EventBeginPlay
  (bind _returnvalue (Game|SpawnActorfromClass "/Game/Blueprints/BP_EnemySpawner.BP_EnemySpawner_C" (Math|Transform|MakeTransform "0, 0,-1000.000000" "0, 0, 0" "1,1,1") "AlwaysSpawn" 0 0))
  (Variables|Default|SetSpawner _returnvalue))

(event EventPostLogin
  (params (NewPlayer :type Player%20Controller%20Object%20Reference))
  ;[1 1 1] onNewClientJoin - add info about new player and update for all connected clients
  (Utilities|Array|Add (Variables|Default|GetplayerControllers) NewPlayer)
  (bind _asin_game_player_controller (Utilities|Casting|CastToInGamePlayerController NewPlayer))
  (Default|Initialize _asin_game_player_controller))

(event EventOnLogout
  (params (ExitingController :type Controller%20Object%20Reference))
  (bind _asplayer_controller (Utilities|Casting|CastToPlayerController ExitingController))
  (|DestroySession _asplayer_controller))

(fn ConstructionScript)

(fn ChoosePlayerStart
  (params (Player :type Controller%20Object%20Reference))
  (bind _outactors (Actor|GetAllActorsOfClass "/Script/Engine.PlayerStart"))
  (bind _array_element (Utilities|Array|ForEachLoopwithBreak _outactors :!label _label)
    (:LoopBody
      (if (Utilities|Name|NotEqual(Name) (Variables|/Script/Engine.PlayerStart|GetPlayerStartTag _array_element) "Taken")
        (Utilities|FlowControl|Sequence
          (:then_0
            (goto _label Break))
          (:then_1
            (Variables|/Script/Engine.PlayerStart|SetPlayerStartTag _array_element "Taken")
            (return _array_element)))))))

(fn ResetPlayers
  (bind _outactors (Actor|GetAllActorsOfClass "/Script/Engine.PlayerStart"))
  (bind _output_get (LocalVariables|SetPlayerStarts _outactors))
  (for _array_element _output_get
    (Variables|/Script/Engine.PlayerStart|SetPlayerStartTag _array_element "Free"))
  (bind _outactors_2 (Actor|GetAllActorsOfClass "/Script/Engine.PlayerController"))
  (for (_array_element_2 _array_index) _outactors_2
    (Transformation|Teleport (Pawn|GetControlledPawn _array_element_2) (Transformation|GetActorLocation (Utilities|Array|Get(acopy) (LocalVariables|GetPlayerStarts) _array_index)) (Transformation|GetActorRotation (Utilities|Array|Get(acopy) (LocalVariables|GetPlayerStarts) _array_index)))
    (bind _asbp_player_ship (Utilities|Casting|CastTobp_PlayerShip (Pawn|GetControlledPawn _array_element_2)))
    (Variables|/Game/Blueprints/bp_Spaceship.bp_Spaceship_C|SetHitPoints _asbp_player_ship (.Value (Utilities|Map|Find (Variables|/Game/Blueprints/BP_ShipParameters.BP_ShipParameters_C|GetCurrentParameters (Variables|/Game/Blueprints/bp_Spaceship.bp_Spaceship_C|GetShipParameters _asbp_player_ship)) "NewEnumerator4")))))

(fn SpawnEnemies
  (bind _numberofenemies (Variables|Default|GetNumberOfEnemies))
  (bind _outactors (Actor|GetAllActorsOfClass "/Game/Blueprints/BP_EnemySpawner.BP_EnemySpawner_C"))
  (LocalVariables|SetEnemiesPerSpawner (/ _numberofenemies (Utilities|Array|Length _outactors)))
  (LocalVariables|SetRemainder (Math|Integer|%(Integer) _numberofenemies (Utilities|Array|Length _outactors)))
  (for _array_element _outactors
    (if (> (LocalVariables|GetRemainder) 0)
      (Default|SpawnWave _array_element (+ (LocalVariables|GetEnemiesPerSpawner) 1))
      (Math|Integer|DecrementInt (LocalVariables|GetRemainder))
      (else
        (Default|SpawnWave _array_element (LocalVariables|GetEnemiesPerSpawner)))))
  (return (Variables|Default|GetNumberOfEnemies)))

(fn GetRandomSpawnPoint
  (return (Math|Transform|MakeTransform (Math|Vector|MakeVector (Math|Random|RandomFloatinRange -1e+03 1e+03) (Math|Random|RandomFloatinRange -1e+03 1e+03) 1e+02) "0, 0, 0" "0.200000,0.200000,0.200000")))

(fn SpawnDefaultPawnfor
  (params (NewPlayer :type Controller%20Object%20Reference) (StartSpot :type Actor%20Object%20Reference))
  (return 0))