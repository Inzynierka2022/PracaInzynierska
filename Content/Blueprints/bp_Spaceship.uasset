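; Player spaceship Blueprint with custom momentum flight, a turret gun and team-aware hit points.
; On server ticks it adds energy along the hull's yaw, applies drag, nudges the energy vector's rotation, then offsets the body by the resulting velocity without sweep.
; Fire input toggles shooting on the BP_TurretPlayer gun.
; Damage from other teams reduces health, destroying gun and ship at zero; the Upgrade event is an empty stub.
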(event Custom|Upgrade
  (params (Type :type UpgradeEnum%20Enum :default "NewEnumerator0"))
  ;[1 1 1] Upgrade
  (switch Utilities|FlowControl|Switch|SwitchonUpgradeEnum Type))

(event Custom|MovePlayer
  (params (Delta%20Seconds :type Float%20%28single-precision%29))
  (bind _spaceshipbody (Variables|Default|GetSpaceshipBody))
  (bind _returnvalue (Transformation|GetWorldRotation _spaceshipbody))
  (Class|CppSpaceship|AddEnergy Delta%20Seconds (.yaw _returnvalue))
  (Class|CppSpaceship|CalculateDragForce (Math|Vector|VectorLength (Variables|Default|GetvelocityVector)))
  (Class|CppSpaceship|CalculateDragVector Delta%20Seconds)
  (Variables|Default|SetenergyVector (+ (Variables|Default|GetenergyVector) (Variables|Default|GetdragVector)))
  (CallFunction|CancelSmallRotationDeviation Delta%20Seconds)
  (Class|CppSpaceship|CalculateVelocityVector (.yaw _returnvalue))
  (Transformation|AddWorldOffset (Variables|Default|GetSpaceshipBody) (Variables|Default|GetvelocityVector) false false))

(event Custom|Fire
  (params (Value :type Boolean))
  ;[1 1 1] Shooting
  (bind _asbp_turret_player (Utilities|Casting|CastToBP_TurretPlayer (Variables|Default|GetGun)))
  (Variables|/Game/Turret/BP_Turret.BP_Turret_C|SetIsShooting _asbp_turret_player Value))

(event EventDamage
  (params (Value :type Integer) (DmgSourceTeam :type Integer))
  (CallFunction|TakeDamage Value DmgSourceTeam))

(event EventTick
  (params (DeltaSeconds :type Float%20%28single-precision%29))
  (if (Networking|IsServer)
    (CallFunction|MovePlayer DeltaSeconds)))

(event Input|ActionEvents|InputActionFire
  (params (Key :type Key%20Structure :default "None"))
  ;[1 1 1] Shooting
  (:Pressed
    (CallFunction|Fire true))
  (:Released
    (CallFunction|Fire false)))

(fn ConstructionScript)

(fn Turn
  (params (Axis%20Value :type Float%20%28single-precision%29))
  (Transformation|AddRelativeRotation (Variables|Default|GetSpaceshipBody) (Math|Rotator|MakeRotator 0.0 0.0 Axis%20Value) false false))

(fn CancelSmallRotationDeviation
  (params (DeltaSeconds :type Float%20%28single-precision%29))
  (Variables|Default|SetenergyVector (Math|Vector|RotateVectorAroundAxis (Variables|Default|GetenergyVector) (* DeltaSeconds 0.1 (Math|Float|Sign(Float) (- (.yaw (Transformation|GetWorldRotation (Variables|Default|GetSpaceshipBody))) (.yaw (Math|Rotator|FindLookatRotation (Math|Vector|MakeVector 0.0 0.0 0.0) (Variables|Default|GetenergyVector)))))) "0, 0,1.000000"))
  (Development|PrintString (Utilities|String|ToString(Float) (- (.yaw (Transformation|GetWorldRotation (Variables|Default|GetSpaceshipBody))) (.yaw (Math|Rotator|FindLookatRotation (Math|Vector|MakeVector 0.0 0.0 0.0) (Variables|Default|GetenergyVector))))) true true "(R=0.000000,G=0.044537,B=1.000000,A=1.000000)" 0.0))

(fn TakeDamage
  (params (Value :type Integer) (DmgSourceTeam :type Integer))
  (if (!= DmgSourceTeam (Variables|Default|GetTeam))
    (bind _output_get (Variables|Default|SetHitPoints (Math|Integer|Clamp(Integer) (- (Variables|Default|GetHitPoints) Value) 0 100)))
    (if (== _output_get 0)
      (Actor|DestroyActor (Variables|Default|GetGun))
      (Actor|DestroyActor))))