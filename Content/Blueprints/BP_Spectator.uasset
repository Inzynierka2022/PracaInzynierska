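; BP_Spectator is a spectator that watches the game through the cameras of player ships.
; Each tick, on authority only, it gathers all Bp_PlayerShip actors and snaps its camera to the selected ship's camera location and rotation.
; Left mouse calls ServerChangePerspective, which advances the selected index, wrapping around the player count.
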(event Custom|ServerChangePerspective
  (Variables|Default|SetSelectedPlayer (Math|Integer|%(Integer) (+ (Variables|Default|GetSelectedPlayer) 1) (Utilities|Array|Length (Variables|Default|GetPlayers)))))

(event EventTick
  (params (DeltaSeconds :type Float%20%28single-precision%29))
  (bind _camera (Variables|Default|GetCamera))
  (Networking|SwitchHasAuthority
    (:Authority
      (bind _outactors (Actor|GetAllActorsOfClass "/Game/Blueprints/bp_PlayerShip.bp_PlayerShip_C"))
      (bind _output_get (Variables|Default|SetPlayers _outactors))
      (if (> (Utilities|Array|Length _output_get) 0)
        (Transformation|SetWorldLocation _camera (Transformation|GetWorldLocation (Variables|/Game/Blueprints/bp_PlayerShip.bp_PlayerShip_C|GetCamera (Utilities|Array|Get(acopy) (Variables|Default|GetPlayers) (Math|Integer|%(Integer) (Variables|Default|GetSelectedPlayer) (Utilities|Array|Length (Variables|Default|GetPlayers)))))) false false)
        (Transformation|SetWorldRotation _camera (Transformation|GetWorldRotation (Variables|/Game/Blueprints/bp_PlayerShip.bp_PlayerShip_C|GetCamera (Utilities|Array|Get(acopy) (Variables|Default|GetPlayers) (Math|Integer|%(Integer) (Variables|Default|GetSelectedPlayer) (Utilities|Array|Length (Variables|Default|GetPlayers)))))) false false)))))

(event Input|MouseEvents|LeftMouseButton
  (params (Key :type Key%20Structure :default "None"))
  (:Pressed
    (CallFunction|ServerChangePerspective)))

(fn ConstructionScript)