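; Medium player ship Blueprint that configures movement, health and turret loadout on top of a parent ship class.
; The construction script feeds max speed, forward thrust and HP from ShipParameters into SetParameters, alongside hard-coded reverse thrust, rotation thrust and drag.
; SpawnTurrets server-spawns two larger and two smaller turrets of one class at arrow components, narrowing the angle limit on all but the first.
; BeginPlay, overlap and Tick only call the parent.
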(event EventBeginPlay
  (|CallParentFunction))

(event Collision|EventActorBeginOverlap
  (params (OtherActor :type Actor%20Object%20Reference))
  (|CallParentFunction OtherActor))

(event EventTick
  (params (DeltaSeconds :type Float%20%28single-precision%29))
  (|CallParentFunction DeltaSeconds))

(fn ConstructionScript
  (bind _shipparameters (Variables|Default|GetShipParameters))
  (bind _baseparameters (Variables|/Game/Blueprints/BP_ShipParameters.BP_ShipParameters_C|GetBaseParameters _shipparameters))
  (|CallParentFunction)
  (CallFunction|SetParameters (.Value (Utilities|Map|Find _baseparameters "NewEnumerator6")) (.Value (Utilities|Map|Find _baseparameters "NewEnumerator10")) 0.5 0.8 1.0 0.2 (.Value (Utilities|Map|Find _baseparameters "NewEnumerator4"))))

(fn SpawnTurrets
  (CallFunction|ServerSpawnTurret "/Game/Blueprints/Turret/Player_Turret/bp_player_turret_medium3.bp_player_turret_medium3_C" 0.15 (Transformation|GetWorldTransform (Variables|Default|GetArrow)))
  (CallFunction|ServerSpawnTurret "/Game/Blueprints/Turret/Player_Turret/bp_player_turret_medium3.bp_player_turret_medium3_C" 0.15 (Transformation|GetWorldTransform (Variables|Default|GetArrow1)))
  (Variables|/Game/Blueprints/Turret/BP_TurretParameters.BP_TurretParameters_C|SetAngleLimit (Variables|/Game/Blueprints/Turret/BP_Turret.BP_Turret_C|GetParameters (Utilities|Array|Get(acopy) (Variables|Default|GetGuns) 1)) 1.6e+02)
  (CallFunction|ServerSpawnTurret "/Game/Blueprints/Turret/Player_Turret/bp_player_turret_medium3.bp_player_turret_medium3_C" 0.1 (Transformation|GetWorldTransform (Variables|Default|GetArrow2)))
  (Variables|/Game/Blueprints/Turret/BP_TurretParameters.BP_TurretParameters_C|SetAngleLimit (Variables|/Game/Blueprints/Turret/BP_Turret.BP_Turret_C|GetParameters (Utilities|Array|Get(acopy) (Variables|Default|GetGuns) 2)) 6e+01)
  (CallFunction|ServerSpawnTurret "/Game/Blueprints/Turret/Player_Turret/bp_player_turret_medium3.bp_player_turret_medium3_C" 0.1 (Transformation|GetWorldTransform (Variables|Default|GetArrow3)))
  (Variables|/Game/Blueprints/Turret/BP_TurretParameters.BP_TurretParameters_C|SetAngleLimit (Variables|/Game/Blueprints/Turret/BP_Turret.BP_Turret_C|GetParameters (Utilities|Array|Get(acopy) (Variables|Default|GetGuns) 3)) 6e+01))