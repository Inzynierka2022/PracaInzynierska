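; Base NPC spaceship that flies itself along a queue of waypoints and reports spawn and destruction to GameplayGamemode as an enemy.
; On the server, Tick moves the ship, draws debug route arrows, turns toward the target and sets gear until each point is reached.
; An exhausted queue stops the ship and calls placeholder route generation, then a clamp toward world origin.
; Helpers build randomized orbital routes, shift or clear them.
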(event Custom|Server%20tick
  (CallFunction|DrawRoutePoints)
  (if (Variables|Default|GetrotationFlag)
    (CallFunction|TurntoTarget)
    (if (Variables|Default|GetautomaticMovementFlag)
      (CallFunction|FollowTargetPoint))))

(event EventBeginPlay
  (|CallParentFunction)
  (Networking|SwitchHasAuthority
    (:Authority
      (CallFunction|StartAutomaticMovement))))

(event Collision|EventActorBeginOverlap
  (params (OtherActor :type Actor%20Object%20Reference)))

(event EventTick
  (params (DeltaSeconds :type Float%20%28single-precision%29))
  (Networking|SwitchHasAuthority
    (:Authority
      (CallFunction|MovePlayer DeltaSeconds)
      (CallFunction|ServerTick))))

(event EventEndPlay
  (params (EndPlayReason :type EEndPlayReason%20Enum :default "Destroyed"))
  (if (Networking|IsServer)
    (bind _asgameplay_gamemode (Utilities|Casting|CastToGameplayGamemode (Game|GetGameMode)))
    (Default|EnemyDestroyed _asgameplay_gamemode)))

(fn ConstructionScript
  (|CallParentFunction)
  (bind _asgameplay_gamemode (Utilities|Casting|CastToGameplayGamemode (Game|GetGameMode)))
  (Default|EnemySpawned _asgameplay_gamemode))

(fn TurntoTarget
  (if (Variables|Default|GetrotationFlag)
    (bind _returnvalue (Class|CppSpaceship|DetermineTurnDirection (.yaw (Transformation|GetWorldRotation (Variables|Default|GetSpaceshipBody))) (.yaw (Math|Rotator|FindLookatRotation (Transformation|GetWorldLocation (Variables|Default|GetSpaceshipBody)) (Variables|Default|GettargetPosition)))))
    (CallFunction|Turn (* _returnvalue (Variables|Default|GetrotationThrusterPower)))))

(fn AngleBetweenPoints
  (params (v1 :type Vector) (v2 :type Vector))
  (return (Class|KismetMathLibrary|DegAcos (Math|Vector|DotProduct (Math|Vector|Normalize v1) (Math|Vector|Normalize v2)))))

(fn FollowTargetPoint
  (if (Variables|Default|GetautomaticMovementFlag)
    (if (< (Math|Vector|VectorLength (- (Transformation|GetWorldLocation (Variables|Default|GetSpaceshipBody)) (Variables|Default|GettargetPosition))) (Variables|Default|GetpathPointAcceptanceDistance))
      (Utilities|Array|RemoveIndex (Variables|Default|GettargetPositionQueue))
      (if (> (Utilities|Array|Length (Variables|Default|GettargetPositionQueue)) 0)
        (Variables|Default|SettargetPosition (Utilities|Array|Get(acopy) (Variables|Default|GettargetPositionQueue)))
        (else
          (Variables|Default|SetautomaticMovementFlag false)
          (Variables|Default|SetrotationFlag false)
          (Variables|Default|SetactualGear 0)
          (CallFunction|ServerGenerateNewRoute)
          (CallFunction|BringTooFarPoints)))
      (elif (not (== (Variables|Default|GetactualGear) 5))
        (Variables|Default|SetactualGear 5)))))

(fn ClearAutomaticMovement
  (Utilities|Array|Clear (Variables|Default|GettargetPositionQueue))
  (Variables|Default|SetautomaticMovementFlag false)
  (Variables|Default|SetrotationFlag false)
  (Variables|Default|SettargetPosition (Transformation|GetWorldLocation (Variables|Default|GetSpaceshipBody))))

(fn AddMovementPoint
  (params (V :type Vector))
  (Utilities|Array|Add (Variables|Default|GettargetPositionQueue) V))

(fn StartAutomaticMovement
  (Variables|Default|SetautomaticMovementFlag true)
  (Variables|Default|SetrotationFlag true))

(fn GeneratePointonCircle
  (params (MiddleOfCircle :type Vector) (Angle :type Float%20%28single-precision%29) (Radius :type Float%20%28single-precision%29))
  (return (+ MiddleOfCircle (Math|Vector|RotateVectorAroundAxis (Math|Vector|MakeVector Radius 0.0 0.0) Angle "0, 0,1.000000"))))

(fn GenerateOrbitalRoute
  (params (Middle :type Vector) (OrbitRadius :type Float%20%28single-precision%29) (NumberOfPoints :type Integer) (InitialOrbitRotation :type Float%20%28single-precision%29) (Orbit%20Fluctuation :type Float%20%28single-precision%29))
  (for _index (range 0 NumberOfPoints)
    (bind _v (CallFunction|GeneratePointonCircle Middle (+ (* _index (/ 3.6e+02 (Math|Conversions|ToFloat(Integer) NumberOfPoints))) InitialOrbitRotation) (+ OrbitRadius (Math|Random|RandomFloatinRange 0.0 Orbit%20Fluctuation))))
    (Utilities|Array|Add (Variables|Default|GettargetPositionQueue) _v)))

(fn DrawRoutePoints
  (Rendering|Debug|DrawDebugArrow (Transformation|GetWorldLocation (Variables|Default|GetSpaceshipBody)) (Variables|Default|GettargetPosition) 2e+01 "(R=1.000000,G=0.779813,B=0.034841,A=1.000000)" 0.0 5.0)
  (for _index (range 0 (- (Utilities|Array|Length (Variables|Default|GettargetPositionQueue)) 2))
    (Rendering|Debug|DrawDebugArrow (Utilities|Array|Get(acopy) (Variables|Default|GettargetPositionQueue) _index) (Utilities|Array|Get(acopy) (Variables|Default|GettargetPositionQueue) (+ _index 1)) 2e+01 "(R=1.000000,G=0.779813,B=0.034841,A=1.000000)" 0.0 5.0)))

(fn FollowNextTarget
  (Utilities|Array|RemoveIndex (Variables|Default|GettargetPositionQueue))
  (if (> (Utilities|Array|Length (Variables|Default|GettargetPositionQueue)) 0)
    (Variables|Default|SettargetPosition (Utilities|Array|Get(acopy) (Variables|Default|GettargetPositionQueue)))
    (else
      (Variables|Default|SetautomaticMovementFlag false)
      (Variables|Default|SetrotationFlag false)
      (Variables|Default|SetactualGear 0))))

(fn MoveRoutePoints
  (params (V :type Vector))
  (bind _targetpositionqueue (Variables|Default|GettargetPositionQueue))
  (Variables|Default|SettargetPosition (+ (Variables|Default|GettargetPosition) V))
  (for (_array_element _array_index) _targetpositionqueue
    (Utilities|Array|SetArrayElem _targetpositionqueue _array_index (+ _array_element V))))

(fn ServerGenerateNewRoute
  (Development|PrintString "Defaul;t route generation" true true "(R=0.000000,G=0.660000,B=1.000000,A=1.000000)" 1.0))

(fn BringTooFarPoints
  (bind _targetpositionqueue (Variables|Default|GettargetPositionQueue))
  ;[1 1 1] Move too far points closer
  (for (_array_element _array_index) _targetpositionqueue
    (if (> (Math|Vector|VectorLength _array_element) 5.5e+03)
      (Class|KismetMathLibrary|VectorSet (Utilities|Array|Get(acopy) _targetpositionqueue _array_index) (.x (Math|Vector|RotateVector (Math|Vector|MakeVector (Math|Random|RandomFloatinRange 4.8e+03 5.5e+03) 0.0 0.0) (Math|Rotator|FindLookatRotation (Math|Vector|MakeVector 0.0 0.0 0.0) _array_element))) (.y (Math|Vector|RotateVector (Math|Vector|MakeVector (Math|Random|RandomFloatinRange 4.8e+03 5.5e+03) 0.0 0.0) (Math|Rotator|FindLookatRotation (Math|Vector|MakeVector 0.0 0.0 0.0) _array_element))) (.z (Math|Vector|RotateVector (Math|Vector|MakeVector (Math|Random|RandomFloatinRange 4.8e+03 5.5e+03) 0.0 0.0) (Math|Rotator|FindLookatRotation (Math|Vector|MakeVector 0.0 0.0 0.0) _array_element))))
      ;[1 1 1] The same but for target position variable
      (if (> (Math|Vector|VectorLength (Variables|Default|GettargetPosition)) 5.5e+03)
        (Variables|Default|SettargetPosition (Math|Vector|MakeVector (.x (Math|Vector|RotateVector (Math|Vector|MakeVector (Math|Random|RandomFloatinRange 4.8e+03 5.5e+03) 0.0 0.0) (Math|Rotator|FindLookatRotation (Math|Vector|MakeVector 0.0 0.0 0.0) (Variables|Default|GettargetPosition)))) (.y (Math|Vector|RotateVector (Math|Vector|MakeVector (Math|Random|RandomFloatinRange 4.8e+03 5.5e+03) 0.0 0.0) (Math|Rotator|FindLookatRotation (Math|Vector|MakeVector 0.0 0.0 0.0) (Variables|Default|GettargetPosition)))) (.z (Math|Vector|RotateVector (Math|Vector|MakeVector (Math|Random|RandomFloatinRange 4.8e+03 5.5e+03) 0.0 0.0) (Math|Rotator|FindLookatRotation (Math|Vector|MakeVector 0.0 0.0 0.0) (Variables|Default|GettargetPosition))))))))))