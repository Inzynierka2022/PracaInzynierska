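; Player controller for a multiplayer spaceship game, owning the HUD, minimap, Tab player list, host console and leave-session flow.
; Upgrade offers up to three random non-maxed upgrades, auto-picking one after a timeout.
; Chosen levels are stored in a map, applied to the ship or its turrets by type, and reapplied on respawn.
; Losing a player ship pawn requests a spectator pawn from the GameplayGamemode.
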(event Custom|Upgrade
  ;[1 1 1] Handling upgrade choice
  (bind _chosen (CallFunction|ChooseUpgradestoShow))
  (if (> (Utilities|Array|Length _chosen) 0)
    (CallFunction|CreateUpgradeWidget _chosen)
    (bind _returnvalue (Utilities|Time|SetTimerbyEvent (delegate Custom|ChooseRandomUpgrade) 15.0))
    (else
      (Development|PrintString "AllUpgradesUnlocked")
      (Default|CallUpgradesFinished))))

(event Custom|UpgradeChosen
  (params (Type :type UpgradeEnum%20Enum :default "NewEnumerator0"))
  (bind _returnvalue (Pawn|GetControlledPawn))
  ;[1 1 1] Applying chosen upgrade to pawn
  (Utilities|Time|ClearandInvalidateTimerbyHandle (stale Custom|Upgrade _returnvalue))
  (CallFunction|DisableUpgradeWidget)
  (bind _level (CallFunction|UpdateUpgrades Type))
  (switch Utilities|FlowControl|Switch|SwitchonUpgradeEnum Type
    (:NewEnumerator0
      (bind _asbp_spaceship (Utilities|Casting|CastTobp_Spaceship _returnvalue :!label _label))
      (for _array_element (Variables|/Game/Blueprints/bp_Spaceship.bp_Spaceship_C|GetGuns _asbp_spaceship)
        (bind _asbp_turret_player (Utilities|Casting|CastToBP_TurretPlayer _array_element))
        (Default|Upgrade _asbp_turret_player Type _level)))
    (:NewEnumerator1
      (goto _label))
    (:NewEnumerator2
      (goto _label))
    (:NewEnumerator3
      (goto _label))
    (:NewEnumerator4
      (bind _asbp_spaceship_2 (Utilities|Casting|CastTobp_Spaceship _returnvalue :!label _label_2))
      (Default|Upgrade _asbp_spaceship_2 Type _level))
    (:NewEnumerator5
      (goto _label))
    (:NewEnumerator6
      (goto _label_2))
    (:NewEnumerator7
      (goto _label))
    (:NewEnumerator9
      (goto _label_2))
    (:NewEnumerator10
      (goto _label_2)))
  (Default|CallUpgradesFinished))

(event Custom|showHUD
  ;[1 1 1] show player HUD
  (bind _returnvalue (UserInterface|CreateWidget "/Game/gui/Hud/playerInGameInterface.playerInGameInterface_C" self))
  (bind _output_get (Variables|Default|SetplayerHud _returnvalue))
  (UserInterface|Viewport|AddtoViewport _output_get 0))

(event Custom|RestoreParametersOnRespawn
  (bind _returnvalue (Pawn|GetControlledPawn))
  (bind _upgradesacquired (Variables|Default|GetUpgradesAcquired))
  ;[1 1 1] Setting ship params after respawn
  (bind _keys (Utilities|Map|Keys _upgradesacquired))
  (for _array_element _keys
    (switch Utilities|FlowControl|Switch|SwitchonUpgradeEnum _array_element
      (:NewEnumerator0
        (bind _asbp_spaceship (Utilities|Casting|CastTobp_Spaceship _returnvalue :!label _label))
        (for _array_element_2 (Variables|/Game/Blueprints/bp_Spaceship.bp_Spaceship_C|GetGuns _asbp_spaceship)
          (bind _asbp_turret_player (Utilities|Casting|CastToBP_TurretPlayer _array_element_2))
          (Default|Upgrade _asbp_turret_player _array_element (.Value (Utilities|Map|Find _upgradesacquired _array_element)))))
      (:NewEnumerator1
        (goto _label))
      (:NewEnumerator2
        (goto _label))
      (:NewEnumerator3
        (goto _label))
      (:NewEnumerator4
        (bind _asbp_spaceship_2 (Utilities|Casting|CastTobp_Spaceship _returnvalue :!label _label_2))
        (Default|Upgrade _asbp_spaceship_2 _array_element (.Value (Utilities|Map|Find _upgradesacquired _array_element))))
      (:NewEnumerator5
        (goto _label))
      (:NewEnumerator6
        (goto _label_2))
      (:NewEnumerator7
        (goto _label))
      (:NewEnumerator9
        (goto _label_2))
      (:NewEnumerator10
        (goto _label_2)))))

(event Custom|leave
  (bind _returnvalue (Game|GetGameMode))
  (bind (_asgameplay_gamemode _bsuccess) (Utilities|Casting|CastToGameplayGamemode _returnvalue))
  ;[1 1 1] updatePlayerListOnLeave
  (Development|PrintString (Utilities|String|ToString(Boolean) _bsuccess) false false)
  (Default|RemovePlayerController _asgameplay_gamemode self))

(event Custom|LocalCreateHud
  ;[1 1 1] Creating Minimap HUD on client
  (bind _returnvalue (UserInterface|CreateWidget "/Game/gui/Minimap/HUD_Widget.HUD_Widget_C" self))
  (bind _output_get (Variables|Default|SetHUD_Widget _returnvalue))
  (UserInterface|Viewport|AddtoViewport _output_get 0))

(event Custom|updatePlayerList
  (params (infos :type Array%20of%20Player%20Info%20Structures))
  ;[1 1 1] updatePlayersList widget content
  (Development|PrintString "updateList" false false "(R=1.000000,G=0.162187,B=0.882185,A=1.000000)" 1e+01)
  (Default|UpdateList (Variables|Default|GetplayersList) infos))

(event Custom|ChooseRandomUpgrade
  ;[1 1 1] Handling upgrade choice
  (CallFunction|UpgradeChosen (Utilities|Array|Get(acopy) (stale Custom|Upgrade _chosen) (Math|Random|RandomIntegerinRange 0 (- (Utilities|Array|Length (stale Custom|Upgrade _chosen)) 1))))
  (CallFunction|DisableUpgradeWidget))

(event Custom|DisableUpgradeWidget
  ;[1 1 1] Disabling upgrade choice menu
  (Widget|RemovefromParent (Variables|Default|GetUpgradeWidget)))

(event Custom|initializePlayersList
  ;[1 1 1] initialize playerList Widget
  (Utilities|IsValid (Variables|Default|GetplayersList)
    (:Is%20Valid
      _)
    (:Is%20Not%20Valid
      (bind _returnvalue (UserInterface|CreateWidget "/Game/gui/Hud/playerList.playerList_C" self))
      (Variables|Default|SetplayersList _returnvalue)
      (UserInterface|Viewport|AddtoViewport (Variables|Default|GetplayersList) 0)))
  (Widget|SetVisibility (Variables|Default|GetplayersList) "Collapsed"))

(event Custom|initialize
  (bind _self self)
  ;[1 1 1] initializeNewPlayerOnJoinToSession
  (CallFunction|ShowHUD _self)
  (CallFunction|InitializePlayersList _self)
  (bind _asonline_game_instance (Utilities|Casting|CastToonlineGameInstance (Game|GetGameInstance)))
  (CallFunction|CallUpdate self (Variables|/Game/gui/PlayerInfo/onlineGameInstance.onlineGameInstance_C|GetplayerInfo _asonline_game_instance)))

(event Custom|CreateUpgradeWidget
  (params (Options :type Array%20of%20UpgradeEnum%20Enums :default "NewEnumerator0"))
  ;[1 1 1] Creating upgrade widget
  (bind _returnvalue (UserInterface|CreateWidget "/Game/gui/Upgrades/UpgradeChoice_Widget.UpgradeChoice_Widget_C" self Options))
  (bind _output_get (Variables|Default|SetUpgradeWidget _returnvalue))
  (UserInterface|Viewport|AddtoViewport _output_get 0))

(event Custom|callUpdate
  (params (newPlayerInfo :type Player%20Info%20Structure))
  ;[1 1 1] callUpdateForNewJoinedPlayer
  (Variables|Default|SetplayerInfo newPlayerInfo)
  (Default|UpdateAll (.AsGameplay%20Gamemode (Utilities|Casting|CastToGameplayGamemode (Game|GetGameMode)))))

(event EventUnPossess
  (params (UnpossessedPawn :type Pawn%20Object%20Reference))
  ;[1 1 1] Sending request for spectator pawn after destroying player pawn
  (Utilities|Casting|CastTobp_PlayerShip UnpossessedPawn)
  (bind _asgameplay_gamemode (Utilities|Casting|CastToGameplayGamemode (Game|GetGameMode)))
  (Default|SpectatorSpawnRequest _asgameplay_gamemode self))

(event EventBeginPlay
  (CallFunction|LocalCreateHud))

(event Input|KeyboardEvents|Tab
  (params (Key :type Key%20Structure :default "None"))
  (:Pressed
    (Utilities|IsValid (Variables|Default|GetplayersList)
      (:Is%20Valid
        _)
      (:Is%20Not%20Valid
        (bind _returnvalue (UserInterface|CreateWidget "/Game/gui/Hud/playerList.playerList_C" self))
        (bind _output_get (Variables|Default|SetplayersList _returnvalue))
        (UserInterface|Viewport|AddtoViewport _output_get 0)))
    (Widget|SetVisibility (Variables|Default|GetplayersList) "Visible"))
  (:Released
    (Widget|SetVisibility (Variables|Default|GetplayersList) "Hidden")))

(event Input|KeyboardEvents|Enter
  (params (Key :type Key%20Structure :default "None"))
  (:Released
    (if (Variables|/Game/gui/PlayerInfo/onlineGameInstance.onlineGameInstance_C|GetisHost (.AsOnline%20Game%20Instance (Utilities|Casting|CastToonlineGameInstance (Game|GetGameInstance))))
      (Utilities|IsValid (Variables|Default|GethostConsole)
        (:Is%20Valid
          (Default|Toggle (Variables|Default|GethostConsole)))
        (:Is%20Not%20Valid
          (bind _returnvalue (UserInterface|CreateWidget "/Game/gui/Hud/hostConsole.hostConsole_C" self))
          (bind _output_get (Variables|Default|SethostConsole _returnvalue))
          (UserInterface|Viewport|AddtoViewport _output_get 0)
          (Default|ShowInput _output_get))))))

(event Input|KeyboardEvents|Q
  (params (Key :type Key%20Structure :default "None"))
  ;[1 1 1] leave game and go to main menu
  (:Pressed
    (CallFunction|Leave)
    (|DestroySession self
      (:OnSuccess
        (Game|OpenLevel(byName) "main_menu")))))

(fn ConstructionScript)

(fn ChooseUpgradestoShow
  (bind _output_get (LocalVariables|SetNumberOfOptions (Math|Integer|Clamp(Integer) (- (|GetNumEnumEntries) (Variables|Default|GetMaxedUpgrades)) 0 3)))
  (while (< (Utilities|Array|Length (LocalVariables|GetChosenUpgrades)) _output_get)
    (while (LocalVariables|GetInvalidUpgrade)
      (LocalVariables|SetTempUpgrade (Utilities|Enum|ByteToEnumUpgradeEnum (Math|Conversions|ToByte(Integer) (Math|Random|RandomIntegerinRange 0 (- (|GetNumEnumEntries) 1)))))
      (LocalVariables|SetInvalidUpgrade (or (>= (.Value (Utilities|Map|Find (Variables|Default|GetUpgradesAcquired) (LocalVariables|GetTempUpgrade))) (Variables|Default|GetMaxUpgradeLevel)) (Utilities|Array|ContainsItem (LocalVariables|GetChosenUpgrades) (LocalVariables|GetTempUpgrade)))))
    (Utilities|Array|Add (LocalVariables|GetChosenUpgrades) (LocalVariables|GetTempUpgrade))
    (LocalVariables|SetInvalidUpgrade true))
  (return (LocalVariables|GetChosenUpgrades)))

(fn UpdateUpgrades
  (params (Type :type UpgradeEnum%20Enum :default "NewEnumerator0"))
  (bind _upgradesacquired (Variables|Default|GetUpgradesAcquired))
  (bind _upgradesacquired_2 (Variables|Default|GetUpgradesAcquired))
  (bind _value (Utilities|Map|Find _upgradesacquired_2 Type))
  (Utilities|Map|Add _upgradesacquired Type (+ (.Value (Utilities|Map|Find _upgradesacquired Type)) 1))
  (if (== _value 5)
    (Math|Integer|IncrementInt (Variables|Default|GetMaxedUpgrades)
      (:%20%20
        _)))
  (return _value))