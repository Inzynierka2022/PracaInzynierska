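; Medium NPC spaceship that carries a turret, patrols, and heads toward players or space stations its radar detects.
; On BeginPlay the server spawns the turret and picks a route: random long patrol if no small NPCs exist, otherwise a fluctuating orbit.
; Radar hits, after a one-second delay, replace the waypoint queue with the target's position and restart automatic movement.
; The construction script sets its flight handling parameters.
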(event OnComponentHit(Radar)
  (params (HitComponent :type Primitive%20Component%20Object%20Reference) (OtherActor :type Actor%20Object%20Reference) (OtherComp :type Primitive%20Component%20Object%20Reference) (NormalImpulse :type Vector :default "0, 0, 0") (Hit :type Hit%20Result%20Structure%20%28by%20ref%29))
  (bind _asbp_player_ship (Utilities|Casting|CastTobp_PlayerShip OtherActor)
    (:then
      (Utilities|FlowControl|Delay 1.0)
      (CallFunction|EnemySpotted! (Transformation|GetWorldLocation (Variables|/Game/Blueprints/bp_Spaceship.bp_Spaceship_C|GetSpaceshipBody _asbp_player_ship))))
    (:CastFailed
      (bind _asbp_space_station (Utilities|Casting|CastTobp_SpaceStation OtherActor))
      (Utilities|FlowControl|Delay 1.0)
      (CallFunction|EnemySpotted! (Transformation|GetWorldLocation (Variables|/Game/Blueprints/bp_Spaceship.bp_Spaceship_C|GetSpaceshipBody _asbp_space_station))))))

(event OnComponentBeginOverlap(Radar)
  (params (OverlappedComponent :type Primitive%20Component%20Object%20Reference) (OtherActor :type Actor%20Object%20Reference) (OtherComp :type Primitive%20Component%20Object%20Reference) (OtherBodyIndex :type Integer) (bFromSweep :type Boolean) (SweepResult :type Hit%20Result%20Structure%20%28by%20ref%29)))

(event EventBeginPlay
  (|CallParentFunction)
  (Networking|SwitchHasAuthority
    (:Authority
      (CallFunction|ServerSpawnTurret "/Game/Blueprints/Turret/NPC_Turret/BP_TurretMedium.BP_TurretMedium_C" 0.15)
      (CallFunction|ServerGenerateNewRoute))))

(event Collision|EventActorBeginOverlap
  (params (OtherActor :type Actor%20Object%20Reference))
  (|CallParentFunction OtherActor))

(event EventTick
  (params (DeltaSeconds :type Float%20%28single-precision%29))
  (|CallParentFunction DeltaSeconds))

(fn ConstructionScript
  (|CallParentFunction)
  (CallFunction|SetParameters 7.0 1.5 0.5 0.8 1.0 0.2 1e+02))

(fn ServerGenerateNewRoute
  (Networking|SwitchHasAuthority
    (:Authority
      (bind _outactors (Actor|GetAllActorsOfClass "/Game/Blueprints/NPC_ships/bp_NPC_Small.bp_NPC_Small_C"))
      (if (== (Utilities|Array|Length _outactors) 0)
        (CallFunction|GenerateLongPatrolRoute 5)
        (else
          (CallFunction|GenerateOrbitalRoute "0, 0, 0" 2.5e+03 8 0.0 2.2e+03)
          (CallFunction|FollowNextTarget)
          (CallFunction|StartAutomaticMovement))))))

(fn GenerateLongPatrolRoute
  (params (NumPoints :type Integer))
  (CallFunction|AddMovementPoint (Math|Vector|RotateVectorAroundAxis (Math|Vector|MakeVector (Math|Random|RandomFloatinRange 5e+02 1.5e+03) 0.0 0.0) (+ (.yaw (Math|Rotator|FindLookatRotation (Transformation|GetWorldLocation (Variables|Default|GetSpaceshipBody)) (Math|Vector|MakeVector 0.0 0.0 0.0))) (Math|Random|RandomFloatinRange -45.0 45.0)) "0, 0,1.000000"))
  (while (< (LocalVariables|GetI) NumPoints)
    (Math|Integer|IncrementInt (LocalVariables|GetI)
      (:%20%20
        (bind _v (CallFunction|GeneratePointonCircle "0, 0, 0" (Math|Random|RandomFloatinRange -1.8e+02 1.8e+02) (Math|Random|RandomFloatinRange 1e+03 3e+03)))
        (CallFunction|AddMovementPoint _v))))
  (CallFunction|StartAutomaticMovement))

(fn EnemySpotted!
  (params (EnemyPosition :type Vector))
  (bind _targetpositionqueue (Variables|Default|GettargetPositionQueue))
  (bind _output_get (Variables|Default|SettargetPosition EnemyPosition))
  (Utilities|Array|Clear _targetpositionqueue)
  (Utilities|Array|Add _targetpositionqueue _output_get)
  (CallFunction|StartAutomaticMovement)
  (Development|PrintString "ENEMY SPOTTED"))