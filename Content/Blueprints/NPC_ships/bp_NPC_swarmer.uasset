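; Small, light NPC swarmer ship that spawns a small turret on the server and wanders through random waypoints around itself.
; Each generated waypoint is nudged toward the world origin, and a new batch is generated when the queue empties.
; At each waypoint it brakes in Tick, then resumes turning toward the next.
; On EndPlay it alerts all swarmers, replacing their routes with its last location.
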(event EventBeginPlay
  (|CallParentFunction)
  (Networking|SwitchHasAuthority
    (:Authority
      (CallFunction|ServerSpawnTurret "/Game/Blueprints/Turret/NPC_Turret/BP_TurretSmall.BP_TurretSmall_C" 0.05)
      (CallFunction|GenerateSwarmingRoute 5e+01 5)
      (CallFunction|StartAutomaticMovement)
      (Variables|Default|SetactualGear 5))))

(event Collision|EventActorBeginOverlap
  (params (OtherActor :type Actor%20Object%20Reference))
  (|CallParentFunction OtherActor))

(event EventTick
  (params (DeltaSeconds :type Float%20%28single-precision%29))
  (|CallParentFunction DeltaSeconds)
  (if (Variables|Default|GetstoppedBetweenPoints)
    (Variables|Default|SetactualGear 0)
    (CallFunction|DecreaseSpeed)
    (if (< (Math|Vector|VectorLength (Variables|Default|GetvelocityVector)) 0.1)
      (Utilities|FlowControl|Delay 1.0)
      (Variables|Default|SetstoppedBetweenPoints false)
      (Variables|Default|SetrotationFlag true))))

(event EventEndPlay
  (params (EndPlayReason :type EEndPlayReason%20Enum :default "Destroyed"))
  (bind _outactors (Actor|GetAllActorsOfClass "bp_NPC_swarmer_C"))
  (for _array_element _outactors
    (CallFunction|RaiseAlert _array_element (Transformation|GetWorldLocation (Variables|Default|GetSpaceshipBody)))))

(fn ConstructionScript
  (|CallParentFunction)
  (CallFunction|SetParameters 1e+01 2.0 0.01 2.0 0.5 0.05 1e+01)
  (Variables|Default|SetpathPointAcceptanceDistance 1.5e+02)
  (CallFunction|FollowNextTarget)
  (Variables|Default|SettargetPosition (Transformation|GetWorldLocation (Variables|Default|GetSpaceshipBody))))

(fn GenerateSwarmingPoint
  (params (Center :type Vector) (minDistance :type Float%20%28single-precision%29) (maxDistance :type Float%20%28single-precision%29))
  (return (+ Center (Math|Vector|RotateVector (* (Math|Vector|MakeVector 1.0 0.0 0.0) (Math|Random|RandomFloatinRange minDistance maxDistance)) (Math|Rotator|MakeRotator 0.0 0.0 (Math|Random|RandomFloatinRange -1.8e+02 1.8e+02))))))

(fn RaiseAlert
  (params (AlertPosition :type Vector))
  (bind _targetpositionqueue (Variables|Default|GettargetPositionQueue))
  (Utilities|Array|Clear _targetpositionqueue)
  (bind _output_get (Variables|Default|SettargetPosition AlertPosition))
  (Utilities|Array|Add _targetpositionqueue _output_get)
  (Variables|Default|SetstoppedBetweenPoints false)
  (CallFunction|StartAutomaticMovement))

(fn GenerateSwarmingRoute
  (params (CloseInDistance :type Float%20%28single-precision%29) (NumPoints :type Integer))
  (while (< (LocalVariables|Geti) NumPoints)
    (Math|Integer|IncrementInt (LocalVariables|Geti)
      (:%20%20
        (bind _swarmpoint (CallFunction|GenerateSwarmingPoint (Transformation|GetWorldLocation (Variables|Default|GetSpaceshipBody)) 2.5e+02 5e+02))
        (Utilities|Array|Add (Variables|Default|GettargetPositionQueue) (+ _swarmpoint (Math|Vector|RotateVector (Math|Vector|MakeVector CloseInDistance 0.0 0.0) (Math|Rotator|MakeRotator 0.0 0.0 (.yaw (Math|Rotator|FindLookatRotation (Transformation|GetWorldLocation (Variables|Default|GetSpaceshipBody)) (Math|Vector|MakeVector 0.0 0.0 0.0))))))))))
  (CallFunction|StartAutomaticMovement))

(fn DecreaseSpeed
  (if (< (Math|Vector|VectorLength (Variables|Default|GetenergyVector)) (Variables|Default|GetreverseThrusterPower))
    (Variables|Default|SetenergyVector "0, 0, 0")
    (else
      (Variables|Default|SetenergyVector (+ (Variables|Default|GetenergyVector) (* (Math|Vector|Normalize (* (Variables|Default|GetenergyVector) -1.0)) (Variables|Default|GetreverseThrusterPower)))))))

(fn FollowTargetPoint
  (if (Variables|Default|GetautomaticMovementFlag)
    (if (< (Math|Vector|VectorLength (- (Transformation|GetWorldLocation (Variables|Default|GetSpaceshipBody)) (Variables|Default|GettargetPosition))) (Variables|Default|GetpathPointAcceptanceDistance))
      (Variables|Default|SetrotationFlag false)
      (Utilities|Array|RemoveIndex (Variables|Default|GettargetPositionQueue))
      (Variables|Default|SetstoppedBetweenPoints true)
      (Variables|Default|SetactualGear 0)
      (if (> (Utilities|Array|Length (Variables|Default|GettargetPositionQueue)) 0)
        _
        (else
          (CallFunction|GenerateSwarmingRoute 1.5e+02 5)))
      (Variables|Default|SettargetPosition (Utilities|Array|Get(acopy) (Variables|Default|GettargetPositionQueue)))
      (elif (not (== (Variables|Default|GetactualGear) (Variables|Default|GetforwardGears)))
        (Variables|Default|SetactualGear (Variables|Default|GetforwardGears))))))