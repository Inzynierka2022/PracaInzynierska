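; Heavy NPC ship that picks a random player ship and continuously orbits it.
; When its waypoint queue is empty, Tick builds a circular route around the target, starting from the ship's current bearing, and starts automatic movement.
; While waypoints remain, it shifts them by the target's movement each tick so the orbit travels with the player.
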(event EventBeginPlay
  (|CallParentFunction) ; This node is disabled and will not be called.\nDrag off pins to build functionality.
)

(event Collision|EventActorBeginOverlap
  (params (OtherActor :type Actor%20Object%20Reference))
  (|CallParentFunction OtherActor) ; This node is disabled and will not be called.\nDrag off pins to build functionality.
)

(event EventTick
  (params (DeltaSeconds :type Float%20%28single-precision%29))
  (|CallParentFunction DeltaSeconds)
  (if (== (Utilities|Array|Length (Variables|Default|GettargetPositionQueue)) 0)
    (if (Variables|Default|GetTargetShipChoosenFlag)
      (CallFunction|GenerateOrbitalRoute (Transformation|GetWorldLocation (Variables|/Game/Blueprints/bp_Spaceship.bp_Spaceship_C|GetSpaceshipBody (Variables|Default|GetchoosenTarget))) 5e+02 25 (.yaw (Math|Rotator|FindLookatRotation (Transformation|GetWorldLocation (Variables|/Game/Blueprints/bp_Spaceship.bp_Spaceship_C|GetSpaceshipBody (Variables|Default|GetchoosenTarget))) (Transformation|GetWorldLocation (Variables|Default|GetSpaceshipBody)))))
      (CallFunction|FollowNextTarget)
      (CallFunction|StartAutomaticMovement)
      (else
        (bind _choosentarget (CallFunction|ChooseTarget :!label _label))
        (bind _output_get (Variables|Default|SetchoosenTarget _choosentarget))
        ;[1 1 1] Used to move orbit with target
        (Variables|Default|SetchoosenTargetPosition (Transformation|GetWorldLocation (Variables|/Game/Blueprints/bp_Spaceship.bp_Spaceship_C|GetSpaceshipBody _output_get)))
        (Variables|Default|SetTargetShipChoosenFlag true)
        (Utilities|Array|Clear (Variables|Default|GettargetPositionQueue))))
    (elif (Variables|Default|GetTargetShipChoosenFlag)
      (CallFunction|MoveRoutePoints (- (Transformation|GetWorldLocation (Variables|/Game/Blueprints/bp_Spaceship.bp_Spaceship_C|GetSpaceshipBody (Variables|Default|GetchoosenTarget))) (Variables|Default|GetchoosenTargetPosition))) ; Move orbit with target
      (Variables|Default|SetchoosenTargetPosition (Transformation|GetWorldLocation (Variables|/Game/Blueprints/bp_Spaceship.bp_Spaceship_C|GetSpaceshipBody (Variables|Default|GetchoosenTarget))))
      (else
        (goto _label)))))

(fn ConstructionScript
  (|CallParentFunction))

(fn ChooseTarget
  (bind _outactors (Actor|GetAllActorsOfClass "/Game/Blueprints/bp_PlayerShip.bp_PlayerShip_C"))
  (return (Utilities|Array|Get(acopy) _outactors (Math|Random|RandomInteger (Utilities|Array|Length _outactors)))))