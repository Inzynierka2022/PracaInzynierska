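; Large NPC spaceship that sets its handling parameters on construction, then on the server spawns a large turret and starts automatic route following.
; While small NPC ships exist it follows a wide, fluctuating orbital route; otherwise it patrols random points around the world origin.
; InformLostScouts rebuilds the route once no small ships remain.
; ChooseTarget returns a random player ship, and EnemySpotted is an empty stub.
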(event EventBeginPlay
  (|CallParentFunction)
  (Networking|SwitchHasAuthority
    (:Authority
      (CallFunction|ServerSpawnTurret "/Game/Blueprints/Turret/NPC_Turret/BP_TurretLarge.BP_TurretLarge_C" 0.05)
      (CallFunction|ServerGenerateNewRoute)
      (CallFunction|FollowNextTarget))))

(event Collision|EventActorBeginOverlap
  (params (OtherActor :type Actor%20Object%20Reference))
  (|CallParentFunction OtherActor) ; This node is disabled and will not be called.\nDrag off pins to build functionality.
)

(event EventTick
  (params (DeltaSeconds :type Float%20%28single-precision%29))
  (|CallParentFunction DeltaSeconds))

(fn ConstructionScript
  (|CallParentFunction)
  (CallFunction|SetParameters 5.0 1e+01 2.0 0.4 5.0 1.0 1e+02))

(fn ChooseTarget
  (bind _outactors (Actor|GetAllActorsOfClass "/Game/Blueprints/bp_PlayerShip.bp_PlayerShip_C"))
  (return (Utilities|Array|Get(acopy) _outactors (Math|Random|RandomInteger (Utilities|Array|Length _outactors)))))

(fn GenerateLongPatrolRoute
  (params (NumPoints :type Integer))
  (CallFunction|AddMovementPoint (Math|Vector|RotateVectorAroundAxis (Math|Vector|MakeVector (Math|Random|RandomFloatinRange 5e+02 1.5e+03) 0.0 0.0) (+ (.yaw (Math|Rotator|FindLookatRotation (Transformation|GetWorldLocation (Variables|Default|GetSpaceshipBody)) (Math|Vector|MakeVector 0.0 0.0 0.0))) (Math|Random|RandomFloatinRange -1e+02 1e+02)) "0, 0,1.000000"))
  (while (< (LocalVariables|GetI) NumPoints)
    (Math|Integer|IncrementInt (LocalVariables|GetI)
      (:%20%20
        (bind _v (CallFunction|GeneratePointonCircle "0, 0, 0" (Math|Random|RandomFloatinRange -1.8e+02 1.8e+02) (Math|Random|RandomFloatinRange 2e+03 4e+03)))
        (CallFunction|AddMovementPoint _v))))
  (CallFunction|StartAutomaticMovement))

(fn ServerGenerateNewRoute
  (Networking|SwitchHasAuthority
    (:Authority
      (bind _outactors (Actor|GetAllActorsOfClass "/Game/Blueprints/NPC_ships/bp_NPC_Small.bp_NPC_Small_C"))
      (if (== (Utilities|Array|Length _outactors) 0)
        (CallFunction|GenerateLongPatrolRoute 5)
        (CallFunction|StartAutomaticMovement)
        (else
          (CallFunction|GenerateOrbitalRoute "0, 0, 0" 5e+03 25 (.yaw (Math|Rotator|FindLookatRotation (Math|Vector|MakeVector 0.0 0.0 0.0) (Transformation|GetWorldLocation (Variables|Default|GetSpaceshipBody)))) 1e+03))))))

(fn InformLostScouts
  (bind _outactors (Actor|GetAllActorsOfClass "/Game/Blueprints/NPC_ships/bp_NPC_Small.bp_NPC_Small_C"))
  (if (== (Utilities|Array|Length _outactors) 0)
    (CallFunction|ClearAutomaticMovement)
    (CallFunction|ServerGenerateNewRoute)))

(fn EnemySpotted!
  (params (EnemyPosition :type Vector)))