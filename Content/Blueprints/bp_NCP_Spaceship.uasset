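; Enemy NPC spaceship that steers toward the player ship and carries an automatic turret.
; On BeginPlay the authority spawns the turret, attaches it to the hull socket and passes it the turret parameters.
; Each tick, ServerTick targets the first player ship found and turns toward it at half input by yaw difference.
; It reports to GameplayGamemode as spawned in the construction script and as destroyed on server EndPlay.
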(event Custom|Server%20tick
  (CallFunction|TurntoTarget)
  (bind _outactors (Actor|GetAllActorsOfClass "/Game/Blueprints/bp_PlayerShip.bp_PlayerShip_C"))
  (CallFunction|TurntoTarget)
  (Variables|Default|SettargetPosition (Transformation|GetWorldLocation (Variables|/Game/Blueprints/bp_Spaceship.bp_Spaceship_C|GetSpaceshipBody (Utilities|Array|Get(acopy) _outactors)))))

(event Custom|ServerSpawnTurret
  (bind _self self)
  (bind _arrow (Variables|Default|GetArrow))
  (bind _returnvalue (Transformation|GetWorldTransform _arrow))
  (bind _returnvalue_2 (Game|SpawnActorfromClass "/Game/Turret/BP_TurretAutomatic.BP_TurretAutomatic_C" (Math|Transform|MakeTransform (.location _returnvalue) (.rotation _returnvalue) "0.300000,0.300000,0.300000") "AlwaysSpawn" _self _self))
  (bind _output_get (Variables|Default|SetGun _returnvalue_2))
  (Transformation|AttachComponentToComponent _output_get (Variables|Default|GetSpaceshipBody) "TurretSocket" "KeepWorld" "SnapToTarget" "KeepWorld" true)
  (Variables|/Game/Turret/BP_Turret.BP_Turret_C|SetParameters _output_get (Variables|Default|GetTurretParameters)))

(event EventBeginPlay
  (|CallParentFunction)
  (Networking|SwitchHasAuthority
    (:Authority
      (CallFunction|ServerSpawnTurret))))

(event Collision|EventActorBeginOverlap
  (params (OtherActor :type Actor%20Object%20Reference)))

(event EventTick
  (params (DeltaSeconds :type Float%20%28single-precision%29))
  (CallFunction|ServerTick))

(event EventEndPlay
  (params (EndPlayReason :type EEndPlayReason%20Enum :default "Destroyed"))
  (if (Networking|IsServer)
    (bind _asgameplay_gamemode (Utilities|Casting|CastToGameplayGamemode (Game|GetGameMode)))
    (Default|EnemyDestroyed _asgameplay_gamemode)))

(fn ConstructionScript
  (|CallParentFunction)
  (bind _asgameplay_gamemode (Utilities|Casting|CastToGameplayGamemode (Game|GetGameMode)))
  (Default|EnemySpawned _asgameplay_gamemode))

(fn TurntoTarget
  (bind _returnvalue (Class|CppSpaceship|DetermineTurnDirection (.yaw (Transformation|GetWorldRotation (Variables|Default|GetSpaceshipBody))) (.yaw (Math|Rotator|FindLookatRotation (Transformation|GetWorldLocation (Variables|Default|GetSpaceshipBody)) (Variables|Default|GettargetPosition)))))
  (CallFunction|Turn (* _returnvalue 0.5)))

(fn AngleBetweenPoints
  (params (v1 :type Vector) (v2 :type Vector))
  (return (Class|KismetMathLibrary|DegAcos (Math|Vector|DotProduct (Math|Vector|Normalize v1) (Math|Vector|Normalize v2)))))