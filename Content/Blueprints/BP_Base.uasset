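; BP_Base is a destructible actor with hit points that can be damaged by any team except team 1.
; Its Damage event passes the value and source team to TakeDamage, which ignores team 1 and subtracts the value from HitPoints, clamped between zero and MaxHitPoints.
; The actor destroys itself when HitPoints reaches zero.
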(event EventDamage
  (params (Value :type Float%20%28single-precision%29) (DmgSourceTeam :type Integer))
  (CallFunction|TakeDamage Value DmgSourceTeam))

(fn ConstructionScript)

(fn TakeDamage
  (params (Value :type Float%20%28single-precision%29) (Team :type Integer))
  (if (!= Team 1)
    (bind _output_get (Variables|Default|SetHitPoints (Math|Float|Clamp(Float) (- (Variables|Default|GetHitPoints) Value) 0.0 (Variables|Default|GetMaxHitPoints))))
    (if (<= _output_get 0.0)
      (Actor|DestroyActor))))