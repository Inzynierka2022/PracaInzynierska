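; GameplayGameState is a game state that mirrors wave progress from GameplayGamemode for a wave-based mode.
; On BeginPlay it copies the max level as MaxWave, then every Tick it polls the game mode for the current wave, enemies left and countdown timer.
; TotalEnemiesLeft has a RepNotify function, which is empty.
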(event EventBeginPlay
  (bind _asgameplay_gamemode (Utilities|Casting|CastToGameplayGamemode (Game|GetGameMode)))
  (Variables|Default|SetMaxWave (Variables|/Game/Blueprints/GameplayGamemode.GameplayGamemode_C|GetMaxLevel _asgameplay_gamemode)))

(event EventTick
  (params (DeltaSeconds :type Float%20%28single-precision%29))
  (bind _asgameplay_gamemode (Utilities|Casting|CastToGameplayGamemode (Game|GetGameMode)))
  (Variables|Default|SetWave (Variables|/Game/Blueprints/GameplayGamemode.GameplayGamemode_C|GetLevel _asgameplay_gamemode))
  (Variables|Default|SetTotal%20Enemies%20Left (Variables|/Game/Blueprints/GameplayGamemode.GameplayGamemode_C|GetTotalEnemiesLeft _asgameplay_gamemode))
  (Variables|Default|SetCountdownTimer (Variables|/Game/Blueprints/GameplayGamemode.GameplayGamemode_C|GetCountdownTimer _asgameplay_gamemode)))

(fn ConstructionScript)

(fn OnRepTotalEnemiesLeft)