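; BP_Bullet is a turret projectile that deals damage on overlap and then destroys itself.
; On overlap it casts the other actor to BP_IDamageable and passes Damage and its TeamId; actors that fail the cast leave the bullet flying.
; The construction script sets the projectile's initial speed from Speed and derives its lifespan from Range divided by that speed, so it expires at maximum range.
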(event Collision|EventActorBeginOverlap
  (params (OtherActor :type Actor%20Object%20Reference))
  (bind _asbp_idamageable (Utilities|Casting|CastToBP_IDamageable OtherActor))
  (Default|Damage _asbp_idamageable (Variables|Default|GetDamage) (Variables|Default|GetTeamId))
  (Actor|DestroyActor))

(fn ConstructionScript
  (bind _output_get (Variables|/Script/Engine.ProjectileMovementComponent|SetInitialSpeed (Variables|Default|GetProjectileMovement) (Variables|Default|GetSpeed)))
  (Actor|SetLifeSpan (/ (Variables|Default|GetRange) _output_get)))