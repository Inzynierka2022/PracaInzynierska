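; BP_TurretAutomatic is an automatic turret that tracks and fires at a player pawn without manual control.
; On BeginPlay, the authority caches the first TestPawn found in the level as its only target.
; Each tick, the authority rotates the turret toward that pawn, calling TryShoot within a fixed distance and StopShooting otherwise.
; Targeting runs only on the authority, and the cached pawn is never refreshed or validity-checked.
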(event EventTick
  (params (DeltaSeconds :type Float%20%28single-precision%29))
  (bind _player (Variables|Default|GetPlayer))
  (bind _returnvalue (Transformation|GetActorTransform _player))
  (|CallParentFunction DeltaSeconds)
  (Networking|SwitchHasAuthority
    (:Authority
      (CallFunction|RotateTowards (.location _returnvalue))
      (if (< (Math|Vector|Distance(Vector) (.location _returnvalue) (Transformation|GetActorLocation)) 1e+03)
        (CallFunction|TryShoot)
        (else
          (CallFunction|StopShooting))))))

(event EventBeginPlay
  (|CallParentFunction)
  (Networking|SwitchHasAuthority
    (:Authority
      (bind _outactors (Actor|GetAllActorsOfClass "/Game/Player/TestPawn.TestPawn_C"))
      (Variables|Default|SetPlayer (Utilities|Array|Get(acopy) _outactors)))))

(fn ConstructionScript
  (|CallParentFunction))