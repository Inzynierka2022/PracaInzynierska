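; Player-controlled turret that aims at the mouse cursor and supports stat upgrades.
; Each tick on a locally controlled pawn, a cursor trace feeds RotateTowards, called directly with authority or via the RequestRotateToMouse event on remote clients.
; Upgrade calls UpgradeParameters, which scales linearly by level from values cached at BeginPlay toward maximums.
; Only fire rate is calculated and printed; the upgrade-type switch has no type-specific logic.
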(event Custom|RequestRotateToMouse
  (params (MousePosition :type Vector))
  (CallFunction|RotateTowards MousePosition))

(event Custom|Upgrade
  (params (Type :type UpgradeEnum%20Enum :default "NewEnumerator0") (Level :type Integer))
  (CallFunction|UpgradeParameters Type Level))

(event EventBeginPlay
  (|CallParentFunction)
  (Variables|Default|SetBaseParameters (Variables|Default|GetParameters)))

(event EventTick
  (params (DeltaSeconds :type Float%20%28single-precision%29))
  (|CallParentFunction DeltaSeconds)
  (Networking|SwitchHasAuthority
    (:Authority
      (bind _aspawn (Utilities|Casting|CastToPawn (Components|GetOwner)))
      (if (Pawn|IsLocallyControlled _aspawn)
        (bind _aspawn_2 (Utilities|Casting|CastToPawn (Components|GetOwner)))
        (bind _asplayer_controller (Utilities|Casting|CastToPlayerController (Pawn|GetController _aspawn_2)))
        (CallFunction|RotateTowards (.Location (Collision|BreakHitResult (.HitResult (Game|Player|GetHitResultUnderCursorbyChannel _asplayer_controller "TraceTypeQuery1" true)))))))
    (:Remote
      (bind _aspawn_3 (Utilities|Casting|CastToPawn (Components|GetOwner)))
      (if (Pawn|IsLocallyControlled _aspawn_3)
        (bind _asplayer_controller_2 (Utilities|Casting|CastToPlayerController (Pawn|GetController _aspawn_3)))
        (CallFunction|RequestRotatetoMouse (.Location (Collision|BreakHitResult (.HitResult (Game|Player|GetHitResultUnderCursorbyChannel _asplayer_controller_2 "TraceTypeQuery1" true)))))))))

(fn ConstructionScript
  (|CallParentFunction))

(fn UpgradeParameters
  (params (Type :type UpgradeEnum%20Enum :default "NewEnumerator0") (Level :type Integer))
  (switch Utilities|FlowControl|Switch|SwitchonUpgradeEnum Type
    (:NewEnumerator0
      _)
    (:NewEnumerator1
      _)
    (:NewEnumerator2
      _)
    (:NewEnumerator3
      _)
    (:NewEnumerator4
      _)
    (:NewEnumerator5
      _)
    (:NewEnumerator6
      _)
    (:NewEnumerator7
      _))
  (bind _output_get (Variables|/Game/BP_TurretParameters.BP_TurretParameters_C|SetFireRate (Variables|Default|GetParameters) (+ (* Level (/ (- (Variables|/Game/BP_TurretParameters.BP_TurretParameters_C|GetFireRate (Variables|Default|GetMaxParameters)) (Variables|/Game/BP_TurretParameters.BP_TurretParameters_C|GetFireRate (Variables|Default|GetBaseParameters))) (Math|Conversions|ToFloat(Integer) (Variables|Default|GetMaxUpgradeLevel)))) (Variables|/Game/BP_TurretParameters.BP_TurretParameters_C|GetFireRate (Variables|Default|GetBaseParameters)))))
  (Development|PrintString (Utilities|String|Append "New fire rate = " (Utilities|String|ToString(Float) _output_get))))