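; Turret actor that fires team-tagged bullets with configurable damage and turns its top toward a target location.
; Tick polls IsShooting; firing spawns BBullet at BulletSpawnPoint, gated by a CanShoot delay plus a one-shot timer at FireRate that is cleared when shooting stops.
; RotateTowards turns RotatableTop at constant speed toward the target's local-space yaw; an angle-limit clamp exists but is unused.
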(event Custom|Shoot
  (CallFunction|Fire)
  (Variables|Default|SetCanShoot false)
  (Utilities|FlowControl|Delay (Variables|Default|GetFireRate))
  (Variables|Default|SetCanShoot true))

(event Custom|TryShoot
  (if (Variables|Default|GetCanShoot)
    (bind _returnvalue (Utilities|Time|SetTimerbyEvent (delegate Custom|Shoot) (Variables|Default|GetFireRate)))
    (CallFunction|Shoot)))

(event Custom|StopShooting
  (Utilities|Time|ClearandInvalidateTimerbyHandle (stale Custom|TryShoot _returnvalue)))

(event EventTick
  (params (DeltaSeconds :type Float%20%28single-precision%29))
  (if (Variables|Default|GetIsShooting)
    (CallFunction|TryShoot)
    (else
      (CallFunction|StopShooting))))

(fn ConstructionScript)

(fn Fire
  (Game|SpawnActorfromClass "/Game/BBullet.BBullet_C" (Transformation|GetWorldTransform (Variables|Default|GetBulletSpawnPoint)) "Undefined" 0 (Variables|Default|GetTeam) (Variables|Default|GetDamage) 0))

(fn RotateTowards
  (params (Target :type Vector%20%28by%20ref%29))
  (Transformation|SetRelativeRotation (Variables|Default|GetRotatableTop) (Class|KismetMathLibrary|RInterptoConstant (.rotation (Transformation|GetRelativeTransform (Variables|Default|GetRotatableTop))) (Math|Rotator|MakeRotator 0.0 0.0 (.yaw (Math|Rotator|MakeRotfromX (Math|Transform|InverseTransformLocation (Transformation|GetActorTransform) Target)))) (Utilities|Time|GetWorldDeltaSeconds) (Variables|Default|GetRotationSpeed)) false false))